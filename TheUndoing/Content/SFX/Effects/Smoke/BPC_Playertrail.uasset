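; Component that provides a toggleable Niagara trail effect on the player's magician character.
; On BeginPlay it spawns the configured system attached to player 0's root component, stores it and keeps it deactivated.
; Start and Stop events activate and deactivate that stored effect, so one instance is reused.
; The spawn passes the capsule's world location as a relative offset.
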(event `self.ReceiveBeginPlay`
  (bind _character (`self.Character`))
  (bind _asbp_magician_player_character (cast `/Game/Player/BP_MagicianPlayerCharacter` (`GameplayStatics.GetPlayerCharacter` 0)))
  (set `self.Character` _asbp_magician_player_character)
  (bind _returnvalue (`NiagaraFunctionLibrary.SpawnSystemAttached` (`self.NiagaraSystem`) (`Actor.RootComponent` _character) "None" (`SceneComponent.K2_GetComponentLocation` (`Character.CapsuleComponent` _character)) (struct) "KeepRelativeOffset" false false))
  (bind _output_get (set `self.Effect` _returnvalue))
  (`self.Deactivate` _output_get))

(event `Start`
  (`self.Activate` (`self.Effect`) false))

(event `Stop`
  (`self.Deactivate` (`self.Effect`)))