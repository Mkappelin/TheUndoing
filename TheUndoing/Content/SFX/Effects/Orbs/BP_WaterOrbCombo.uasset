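; BP_WaterOrbCombo is a water orb projectile actor, launched through its Shooting event.
; While shooting, Tick moves it along its forward vector at Speed with a swept world offset.
; On a blocking hit it spawns a water splash actor and impact sound at the collider, then destroys itself.
; A disconnected branch that would resolve the magician player's active event spell never runs.
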(event `Shooting`
  (set `self.IsShooting` true))

(event `self.ReceiveTick`
  (params (DeltaSeconds :type "Float (single-precision)"))
  (bind _returnvalue (`SceneComponent.K2_GetComponentLocation` (`self.OrbCollider`)))
  (if (`self.IsShooting`)
    (bind _sweephitresult (`self.K2_AddActorWorldOffset` (* DeltaSeconds (`self.GetActorForwardVector`) (`self.Speed`)) true))
    (if (`GameplayStatics.BreakHitResult` _sweephitresult)
      (`|SpawnActorFromClass` "/Game/SFX/Effects/Damage/BP_WATERSPLASH.BP_WATERSPLASH_C" (`KismetMathLibrary.Conv_VectorToTransform` _returnvalue) "Undefined" "MultiplyWithRoot" null null)
      (`GameplayStatics.SpawnSoundAtLocation` "/Game/Sounds/WaterImpact__2_.WaterImpact__2_" _returnvalue (struct) 0.2 1.2 0.0 null null)
      (set `self.IsShooting` false)
      (`self.K2_DestroyActor`))))

(fn `UserConstructionScript`)