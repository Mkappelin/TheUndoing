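; BP_ForceOrb is a projectile orb for the magician player's force spell.
; Each tick it moves forward along its facing at Speed using a swept offset.
; On a blocking hit it spawns BP_ForceEffect at the collider, calls ResolveSpell on the player character's ActiveEvent, then destroys itself.
; If the player is not a BP_MagicianPlayerCharacter, the cast fails and the orb is not destroyed.
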(event `self.ReceiveTick`
  (params (DeltaSeconds :type "Float (single-precision)"))
  (bind _sweephitresult (`self.K2_AddActorWorldOffset` (* DeltaSeconds (`self.GetActorForwardVector`) (`self.Speed`)) true))
  (if (`GameplayStatics.BreakHitResult` _sweephitresult)
    (`|SpawnActorFromClass` "/Game/SFX/Effects/Damage/BP_ForceEffect.BP_ForceEffect_C" (`KismetMathLibrary.Conv_VectorToTransform` (`SceneComponent.K2_GetComponentLocation` (`self.OrbCollider`))) "Undefined" "MultiplyWithRoot" null null)
    (bind _asbp_magician_player_character (cast `/Game/Player/BP_MagicianPlayerCharacter` (`GameplayStatics.GetPlayerCharacter` 0)))
    (`/Game/Blueprints/Events/BP_EventMaster.ResolveSpell` (`/Game/Player/BP_MagicianPlayerCharacter.ActiveEvent` _asbp_magician_player_character))
    (`self.K2_DestroyActor`)))

(fn `UserConstructionScript`)