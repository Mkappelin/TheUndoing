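; BP_FirballCombo is a fireball projectile actor that, once its Shooting event fires, flies along its forward vector at Speed.
; Tick moves it with a swept world offset while IsShooting is set.
; On a blocking hit it spawns BP_FIRE_FX and an impact sound at the fireball's location, then destroys itself.
; An unconnected branch would call ResolveSpell on the magician player's ActiveEvent, but it never runs.
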(event `Shooting`
  (set `self.IsShooting` true))

(event `self.ReceiveTick`
  (params (DeltaSeconds :type "Float (single-precision)"))
  (bind _returnvalue (`SceneComponent.K2_GetComponentLocation` (`self.FIREBALL`)))
  (if (`self.IsShooting`)
    (bind _sweephitresult (`self.K2_AddActorWorldOffset` (* DeltaSeconds (`self.GetActorForwardVector`) (`self.Speed`)) true))
    (if (`GameplayStatics.BreakHitResult` _sweephitresult)
      (`|SpawnActorFromClass` "/Game/SFX/Effects/Damage/BP_FIRE_FX.BP_FIRE_FX_C" (`KismetMathLibrary.Conv_VectorToTransform` _returnvalue) "Undefined" "MultiplyWithRoot" null null)
      (`GameplayStatics.SpawnSoundAtLocation` "/Game/Sounds/FireImpact.FireImpact" _returnvalue (struct) 0.25 1.0 0.0 null null)
      (set `self.IsShooting` false)
      (`self.K2_DestroyActor`))))

(fn `UserConstructionScript`)