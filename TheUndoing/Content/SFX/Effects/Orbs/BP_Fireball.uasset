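; BP_Fireball is a projectile actor that flies along its forward vector and bursts into a fire effect on impact.
; Each tick it moves by Speed scaled by delta time using a swept world offset rather than a projectile movement component.
; A blocking hit spawns BP_FIRE_FX at the FIREBALL component's location and destroys the actor, with no damage applied in these graphs.
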(event `self.ReceiveBeginPlay`)

(event `self.ReceiveTick`
  (params (DeltaSeconds :type "Float (single-precision)"))
  (bind _sweephitresult (`self.K2_AddActorWorldOffset` (* DeltaSeconds (`self.GetActorForwardVector`) (`self.Speed`)) true))
  (if (`GameplayStatics.BreakHitResult` _sweephitresult)
    (`|SpawnActorFromClass` "/Game/SFX/Effects/Damage/BP_FIRE_FX.BP_FIRE_FX_C" (`KismetMathLibrary.Conv_VectorToTransform` (`SceneComponent.K2_GetComponentLocation` (`self.FIREBALL`))) "Undefined" "MultiplyWithRoot" null null)
    (`self.K2_DestroyActor`)))

(fn `UserConstructionScript`)