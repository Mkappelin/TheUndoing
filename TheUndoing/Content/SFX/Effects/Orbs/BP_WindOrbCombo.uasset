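; BP_WindOrbCombo is a wind orb projectile actor that starts flying forward once Shooting is triggered.
; Tick moves it along its forward vector at Speed using a swept offset.
; On a blocking hit it spawns BP_WindEffect at the collider, plays a sound there and destroys itself.
; An unconnected chain that would resolve the magician player's active spell before destruction never runs.
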(event `Shooting`
  (set `self.IsShooting` true))

(event `self.ReceiveTick`
  (params (DeltaSeconds :type "Float (single-precision)"))
  (bind _returnvalue (`SceneComponent.K2_GetComponentLocation` (`self.OrbCollider`)))
  (if (`self.IsShooting`)
    (bind _sweephitresult (`self.K2_AddActorWorldOffset` (* DeltaSeconds (`self.GetActorForwardVector`) (`self.Speed`)) true))
    (if (`GameplayStatics.BreakHitResult` _sweephitresult)
      (`|SpawnActorFromClass` "/Game/SFX/Effects/Damage/BP_WindEffect.BP_WindEffect_C" (`KismetMathLibrary.Conv_VectorToTransform` _returnvalue) "Undefined" "MultiplyWithRoot" null null)
      (`GameplayStatics.PlaySoundAtLocation` null _returnvalue (struct) 1.0 1.0 0.0 null null null null)
      (set `self.IsShooting` false)
      (`self.K2_DestroyActor`))))

(fn `UserConstructionScript`)