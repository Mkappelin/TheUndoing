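; BP_SpellEventBurningHouse is a trigger actor for a burning-house spell-casting event.
; When the player character overlaps CollisionEnter, SetupEvent switches the magician controller into paint mode with a blended camera and binds to spell recognition.
; It teleports the player to PlayerPos and aims control rotation at PointOfInterest, printing that rotation.
; The OnSpell and OnEnterEvent handlers are empty, so spell results have no effect here.
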(event `self.CollisionEnter.OnComponentBeginOverlap`
  (params (OverlappedComponent :type "PrimitiveComponent Object Reference") (OtherActor :type "Actor Object Reference") (OtherComp :type "PrimitiveComponent Object Reference") (OtherBodyIndex :type Integer) (bFromSweep :type Boolean) (SweepResult :type "HitResult Structure (by ref)"))
  (if (== OtherActor (`GameplayStatics.GetPlayerCharacter` 0))
    (`self.SetupEvent`)))

(event `OnEnterEvent`)

(event `OnSpell`
  (params (Result :type "SpellRecognitionResult Structure (by ref)")))

(fn `SetupEvent`
  (bind _returnvalue (`SceneComponent.K2_GetComponentLocation` (`self.PlayerPos`)))
  (bind _returnvalue_2 (`KismetMathLibrary.FindLookAtRotation` _returnvalue (`SceneComponent.K2_GetComponentLocation` (`self.Point of Interest`))))
  (bind _asbp_magician_player_controller (cast `/Game/Player/BP_MagicianPlayerController` (`GameplayStatics.GetPlayerController` 0)))
  (`MagicianPlayerController.EnterPaintMode` _asbp_magician_player_controller (`ActorComponent.GetOwner` (`self.Camera`)) 0.5)
  (add `MagicianPlayerController.OnSpellRecognized` _asbp_magician_player_controller (`|CreateDelegate` :!event `OnSpell`))
  (`self.K2_TeleportTo` :`self` (`GameplayStatics.GetPlayerCharacter` 0) :`DestLocation` _returnvalue)
  (`Controller.SetControlRotation` (`GameplayStatics.GetPlayerController` 0) _returnvalue_2)
  (`KismetSystemLibrary.PrintString` (`KismetStringLibrary.Conv_RotatorToString` _returnvalue_2)))

(fn `UserConstructionScript`)