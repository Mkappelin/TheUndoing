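; Combat manager for drawn-spell battles: on enemy contact it moves the player into position, enters paint mode and shows the HUD.
; Recognised spells set accuracy-scaled damage and cast, Shield grants a timed block, and combo mode chains up to four spells with pairwise damage multipliers.
; A Tick countdown triggers enemy attacks, with the next timer chosen by AI type and blocks reducing damage by accuracy.
; Either death ends combat and restores player health.
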(event `self.ReceiveBeginPlay`)

(event `self.ReceiveTick`
  (params (DeltaSeconds :type "Float (single-precision)"))
  (if (`self.InCombat`)
    (`self.TimerEvent1`)
    (if (`self.IsBlock`)
      (`self.BlockTImerEvent`))
    (if (== (`self.Timer`) 0.0)
      (`self.EnemyAttack1`))
    (`KismetSystemLibrary.Delay` 1.0)))

(event `EnemyCollided`
  (params (`Enemy refrence` :type "/Game/Blueprints/BP_Enemy Object Reference") (Timer :type "Float (double-precision)") (`AI type` :type Integer) (`Enemy Damage` :type "Float (double-precision)"))
  (bind _returnvalue (`GameplayStatics.GetPlayerCharacter` 0))
  (bind _enemy1 (`self.Enemy1`))
  (bind _returnvalue_2 (`SceneComponent.K2_GetComponentLocation` (`/Game/Blueprints/BP_Enemy.PlayerPos` _enemy1)))
  (`self.BindEnemy1` `Enemy refrence`)
  (set `self.InitialTImer` Timer)
  (set `self.EnemyAI` `AI type`)
  (set `self.EnemyDMG` `Enemy Damage`)
  (bind _asbp_magician_player_character (cast `/Game/Player/BP_MagicianPlayerCharacter` _returnvalue))
  (`/Game/Player/BP_MagicianPlayerCharacter.BindActiveEvent` _asbp_magician_player_character self)
  (`/Game/Player/BP_MagicianPlayerCharacter.EnemyOverlap` _asbp_magician_player_character `Enemy refrence`)
  (bind _asbp_magician_player_controller (cast `/Game/Player/BP_MagicianPlayerController` (`GameplayStatics.GetPlayerController` 0)))
  (`MagicianPlayerController.EnterPaintMode` _asbp_magician_player_controller (`ActorComponent.GetOwner` (`/Game/Blueprints/BP_Enemy.Camera` _enemy1)) 0.5)
  (add `MagicianPlayerController.OnSpellRecognized` _asbp_magician_player_controller (`|CreateDelegate` :!event `OnSpell`))
  (`self.K2_TeleportTo` :`self` _returnvalue :`DestLocation` _returnvalue_2)
  (`SceneComponent.K2_SetWorldRotation` (`Character.CapsuleComponent` (`GameplayStatics.GetPlayerCharacter` 0)) (`KismetMathLibrary.MakeRotator` 0.0 0.0 (.yaw (`KismetMathLibrary.FindLookAtRotation` _returnvalue_2 (`SceneComponent.K2_GetComponentLocation` (`Actor.RootComponent` _enemy1))))) false false)
  (`self.BattleBegin1`))

(event `PlayerBlock`
  (set `self.IsBlock` true))

(event `BlockTImerEvent`
  (bind _output_get (set `self.BlockTimer` (`KismetMathLibrary.FClamp` (- (`self.BlockTimer`) (stale `self.ReceiveTick` DeltaSeconds)) 0.0 (`self.BlockTimer`))))
  (if (== _output_get 0.0)
    (set `self.IsBlock` false)
    (set `self.BlockTimer` 1.25)))

(event `OnSpell`
  (params (Result :type "SpellRecognitionResult Structure (by ref)"))
  (bind (_bsuccess _name _score) (break `SpellRecognitionResult` Result))
  (set `self.Accuracy` _score)
  (`KismetSystemLibrary.PrintString` (`KismetStringLibrary.Concat_StrStr` "Spell Success: " (`KismetStringLibrary.Conv_BoolToString` _bsuccess) ", Shape: " _name ", Score: " (`KismetStringLibrary.Conv_DoubleToString` _score)) true true (struct :`G` 0.66 :`B` 1.0 :`A` 1.0) 5.0)
  (switch `string` _name
    (:`Fire`
      (set `self.RecognizedSpell` "NewEnumerator1")
      (if (`self.Combo`) :!label _label
        (`self.ComboCalc` Result (`self.RecognizedSpell`))
        (else
          (set `self.PlayerDMG` (* (`self.Accuracy`) (`self.PlayerDMGOriginal`)))
          (bind _asbp_magician_player_character (cast `/Game/Player/BP_MagicianPlayerCharacter` (`GameplayStatics.GetPlayerCharacter` 0)))
          (`/Game/Player/BP_MagicianPlayerCharacter.CastSpell` _asbp_magician_player_character (`SceneComponent.K2_GetComponentLocation` (`Actor.RootComponent` (`self.Enemy1`))) (`self.RecognizedSpell`) (`self.InCombat`)))))
    (:`Water`
      (set `self.RecognizedSpell` "NewEnumerator0")
      (goto _label))
    (:`Lightning`
      (set `self.RecognizedSpell` "NewEnumerator2")
      (goto _label))
    (:`Lifting`
      (set `self.RecognizedSpell` "NewEnumerator4")
      (goto _label))
    (:`Shield`
      (`self.BlockEffect`)
      (`self.PlayerBlock`))))

(event `ComboON`
  (`KismetSystemLibrary.PrintString` "COMBO ON")
  (set `self.Combo` true))

(event `ComboOFF`
  (`KismetSystemLibrary.PrintString` "COMBO OFF")
  (`self.ComboShoot`))

(fn `BattleBegin1`
  (set `self.IsBlock` false)
  (set `self.Timer` 6.0)
  (set `self.InCombat` true)
  (`KismetSystemLibrary.PrintString` "battle started")
  (bind _asbp_magician_player_character (cast `/Game/Player/BP_MagicianPlayerCharacter` (`GameplayStatics.GetPlayerCharacter` 0)))
  (bind _output_get (set `self.PlayerHUDRef` (`/Game/Player/BP_MagicianPlayerCharacter.HUDRef` _asbp_magician_player_character)))
  (set `Widget.Visibility` "Visible" _output_get)
  (`KismetSystemLibrary.PrintString` "HUD Visable"))

(fn `BindEnemy1`
  (params (Enemy :type "/Game/Blueprints/BP_Enemy Object Reference"))
  (set `self.Enemy1` Enemy))

(fn `BlockEffect`
  (`|SpawnActorFromClass` "/Game/SFX/Effects/Shield/BP_Shield.BP_Shield_C" (`KismetMathLibrary.Conv_VectorToTransform` (`SceneComponent.K2_GetComponentLocation` (`/Game/Blueprints/BP_Enemy.sHIELD Pos` (`self.Enemy1`)))) "Undefined" "MultiplyWithRoot" null null))

(fn `ComboCalc`
  (params (Result :type "SpellRecognitionResult Structure") (`Spell ` :type "/Game/Blueprints/Spells Enum" :default "NewEnumerator0"))
  (bind (_bsuccess _name _score) (break `SpellRecognitionResult` Result))
  (bind _accuracy (`self.Accuracy`))
  (bind _combospells (`self.ComboSpells`))
  (bind _returnvalue (+ (* (`self.PlayerDMGOriginal`) _accuracy) (* (`self.PlayerDMG`) _accuracy)))
  (`KismetSystemLibrary.PrintString` "WE COMBOING")
  (set `self.Accuracy` _score)
  (switch `string` (`self.PreviousSpell`)
    (:`Default`
      _)
    (:`Fire`
      (switch `/Game/Blueprints/Spells` `Spell `
        (:`NewEnumerator0`
          (set `self.PlayerDMG` (* _returnvalue 0.5)))
        (:`NewEnumerator1`
          (set `self.PlayerDMG` (* _returnvalue 1.2)))
        (:`NewEnumerator2`
          (set `self.PlayerDMG` (* _returnvalue 0.9)))
        (:`NewEnumerator4`
          (set `self.PlayerDMG` (* _returnvalue 1.5)))))
    (:`Water`
      (switch `/Game/Blueprints/Spells` `Spell `
        (:`NewEnumerator0`
          (set `self.PlayerDMG` (* _returnvalue 1.2)))
        (:`NewEnumerator1`
          (set `self.PlayerDMG` (* _returnvalue 0.5)))
        (:`NewEnumerator2`
          (set `self.PlayerDMG` (* _returnvalue 1.5)))
        (:`NewEnumerator4`
          (set `self.PlayerDMG` (* _returnvalue 1.1)))))
    (:`Lightning`
      (switch `/Game/Blueprints/Spells` `Spell `
        (:`NewEnumerator0`
          (set `self.PlayerDMG` (* _returnvalue 1.1)))
        (:`NewEnumerator1`
          (set `self.PlayerDMG` (* _returnvalue 1.0)))
        (:`NewEnumerator2`
          (set `self.PlayerDMG` (* _returnvalue 1.2)))
        (:`NewEnumerator4`
          (set `self.PlayerDMG` (* _returnvalue 1.0)))))
    (:`Lifting`
      (switch `/Game/Blueprints/Spells` `Spell `
        (:`NewEnumerator0`
          (set `self.PlayerDMG` (* _returnvalue 1.1)))
        (:`NewEnumerator1`
          (set `self.PlayerDMG` (* _returnvalue 1.1)))
        (:`NewEnumerator2`
          (set `self.PlayerDMG` (* _returnvalue 1.0)))
        (:`NewEnumerator4`
          (set `self.PlayerDMG` (* _returnvalue 1.3))))))
  (set `self.PreviousSpell` _name)
  (`KismetArrayLibrary.Array_Add` (`self.ComboSpells`) `Spell `)
  (bind _asbp_magician_player_character (cast `/Game/Player/BP_MagicianPlayerCharacter` (`GameplayStatics.GetPlayerCharacter` 0)))
  (`/Game/Player/BP_MagicianPlayerCharacter.SpawnSpellProjectileCombo` _asbp_magician_player_character (`SceneComponent.K2_GetComponentLocation` (`Actor.RootComponent` (`self.Enemy1`))) (`self.RecognizedSpell`) _combospells)
  (if (== 4 (`KismetArrayLibrary.Array_Length` _combospells))
    (`self.ComboShoot`)))

(fn `ComboShoot`
  (set `self.Combo` false)
  (if (== (`self.PreviousSpell`) "null")
    (return)
    (else
      (bind _asbp_magician_player_character (cast `/Game/Player/BP_MagicianPlayerCharacter` (`GameplayStatics.GetPlayerCharacter` 0)))
      (`/Game/Player/BP_MagicianPlayerCharacter.ComboAnimation` _asbp_magician_player_character)
      (set `self.PreviousSpell` "null")
      (`KismetArrayLibrary.Array_Clear` (`self.ComboSpells`)))))

(fn `EnemyAttack1`
  (returns (ReturnValue :type "PlayerController Object Reference"))
  (bind _returnvalue (`GameplayStatics.GetPlayerCharacter` 0))
  (`/Game/Blueprints/BP_Enemy.OnAttack` (`self.Enemy1`))
  (bind _asbp_magician_player_character (cast `/Game/Player/BP_MagicianPlayerCharacter` _returnvalue))
  (switch `int` (`self.EnemyAI`)
    (:`Default`
      (bind _output_get (set `self.Timer` (`self.InitialTImer`)))
      (bind _statscomp (`/Game/Player/BP_MagicianPlayerCharacter.StatsComp` _asbp_magician_player_character))
      (set `/Game/Blueprints/BP_StatsComponent.CombatTimerDuration` _output_get _statscomp))
    (:`0`
      (bind _timerout (`self.SimpleAI` 0.0))
      (set `/Game/Blueprints/BP_StatsComponent.CombatTimerDuration` _timerout _statscomp))
    (:`1`
      (bind _returnvalue_2 (`EnemyAttackBehaviorTree.CalculateAttackTimerDirect` (`self.Previous timer`) (`KismetMathLibrary.FTrunc` (`/Game/Blueprints/BP_StatsComponent.CurrentHealth` (`/Game/Blueprints/BP_Enemy.BP_StatsComponent` (`self.Enemy1`)))) 0 (`self.IsBlock`) (`self.AttackAccuracy`)))
      (bind _output_get_2 (set `self.Timer` _returnvalue_2))
      (`KismetSystemLibrary.PrintString` (`KismetStringLibrary.Conv_DoubleToString` _output_get_2))
      (set `/Game/Blueprints/BP_StatsComponent.CombatTimerDuration` _output_get_2 _statscomp)
      (set `self.Previous timer` _output_get_2)))
  (bind _asbp_magician_player_character_2 (cast `/Game/Player/BP_MagicianPlayerCharacter` _returnvalue))
  (if (`self.IsBlock`)
    (bind _statscomp_2 (`/Game/Player/BP_MagicianPlayerCharacter.StatsComp` _asbp_magician_player_character_2))
    (`/Game/Blueprints/BP_StatsComponent.TakeDamageSimple` _statscomp_2 (* (`self.EnemyDMG`) (- 1.0 (`self.Accuracy`))))
    (else
      (`/Game/Blueprints/BP_StatsComponent.TakeDamageSimple` _statscomp_2 (`self.EnemyDMG`))))
  (`|SpawnActorFromClass` "/Game/SFX/Effects/Damage/BP_Damage_FX.BP_Damage_FX_C" (`KismetMathLibrary.Conv_VectorToTransform` (`SceneComponent.K2_GetComponentLocation` (`Actor.RootComponent` (`GameplayStatics.GetPlayerCharacter` 0)))) "Undefined" "MultiplyWithRoot" null null)
  (set `self.IsBlock` false)
  (if (== (`/Game/Blueprints/BP_StatsComponent.GetHealthPercent` (`/Game/Player/BP_MagicianPlayerCharacter.StatsComp` _asbp_magician_player_character_2)) 0.0)
    (`self.PlayerDeath1`)))

(fn `EnemyDeath1`
  (bind _asbp_magician_player_controller (cast `/Game/Player/BP_MagicianPlayerController` (`GameplayStatics.GetPlayerController` 0)))
  (set `MagicianPlayerController.bIsPaintingMode` true _asbp_magician_player_controller)
  (`MagicianPlayerController.ExitPaintMode` _asbp_magician_player_controller 0.5)
  (set `self.InCombat` false)
  (`self.K2_DestroyActor` (`self.Enemy1`))
  (bind _asbp_magician_player_character (cast `/Game/Player/BP_MagicianPlayerCharacter` (`GameplayStatics.GetPlayerCharacter` 0)))
  (bind _statscomp (`/Game/Player/BP_MagicianPlayerCharacter.StatsComp` _asbp_magician_player_character))
  (set `/Game/Blueprints/BP_StatsComponent.CurrentHealth` (`/Game/Blueprints/BP_StatsComponent.MaxHealth` _statscomp) _statscomp)
  (set `Widget.Visibility` "Collapsed" (`self.PlayerHUDRef`))
  (`KismetSystemLibrary.PrintString` "HUD Visable"))

(fn `FireEffect`
  (bind _returnvalue (`|SpawnActorFromClass` "/Game/SFX/Effects/Beams/BP_Firebeam.BP_Firebeam_C" (`KismetMathLibrary.Conv_VectorToTransform` (`SceneComponent.K2_GetComponentLocation` (`/Game/Blueprints/BP_Enemy.AtkAnimPos` (`self.Enemy1`)))) "Undefined" "MultiplyWithRoot" self null))
  (bind _returnvalue_2 (`self.GetTargetRotation`))
  (`SceneComponent.K2_SetWorldRotation` (`/Game/SFX/Effects/Beams/BP_Firebeam.DefaultSceneRoot` _returnvalue) _returnvalue_2 false false)
  (`|SpawnActorFromClass` "/Game/SFX/Effects/Damage/BP_Damage_FX.BP_Damage_FX_C" (`KismetMathLibrary.Conv_VectorToTransform` (`SceneComponent.K2_GetComponentLocation` (`/Game/Blueprints/BP_Enemy.Sphere` (`self.Enemy1`)))) "Undefined" "MultiplyWithRoot" null null))

(fn `GetTargetRotation`
  (returns (ReturnValue :type "Rotator Structure"))
  (bind _enemy1 (`self.Enemy1`))
  (return (`KismetMathLibrary.MakeRotator` 0.0 0.0 (.yaw (`KismetMathLibrary.FindLookAtRotation` (`SceneComponent.K2_GetComponentLocation` (`/Game/Blueprints/BP_Enemy.AtkAnimPos` _enemy1)) (`SceneComponent.K2_GetComponentLocation` (`/Game/Blueprints/BP_Enemy.Sphere` _enemy1)))))))

(fn `PlayerAttack1`
  (bind _bp_statscomponent (`/Game/Blueprints/BP_Enemy.BP_StatsComponent` (`self.Enemy1`)))
  (bind _currenthealth (`/Game/Blueprints/BP_StatsComponent.CurrentHealth` _bp_statscomponent))
  (if (`self.PlayerTurn`)
    (set `self.AttackAccuracy` (`self.Accuracy`))
    (`/Game/Blueprints/BP_StatsComponent.TakeDamageSimple` _bp_statscomponent (`self.PlayerDMG`))
    (`/Game/Blueprints/BP_Enemy.TakeDamage` (`self.Enemy1`) (>= (`self.AttackAccuracy`) 0.9) (`self.PlayerDMG`) (`self.RecognizedSpell`))
    (`KismetSystemLibrary.PrintString` (`KismetStringLibrary.Conv_DoubleToString` _currenthealth))
    (`|SpawnActorFromClass` "/Game/SFX/Effects/Damage/BP_Damage_FX.BP_Damage_FX_C" (`KismetMathLibrary.Conv_VectorToTransform` (`SceneComponent.K2_GetComponentLocation` (`Character.Mesh` (`self.Enemy1`)))) "Undefined" "MultiplyWithRoot" null null)
    (set `self.PlayerDMG` (`self.PlayerDMGOriginal`))
    (if (<= _currenthealth 0.0)
      (`self.EnemyDeath1`))))

(fn `PlayerDeath1`
  (bind _bp_statscomponent (`/Game/Blueprints/BP_Enemy.BP_StatsComponent` (`self.Enemy1`)))
  (bind _asbp_magician_player_controller (cast `/Game/Player/BP_MagicianPlayerController` (`GameplayStatics.GetPlayerController` 0)))
  (set `MagicianPlayerController.bIsPaintingMode` true _asbp_magician_player_controller)
  (`MagicianPlayerController.ExitPaintMode` _asbp_magician_player_controller 0.5)
  (set `self.InCombat` false)
  (bind _asbp_magician_player_character (cast `/Game/Player/BP_MagicianPlayerCharacter` (`GameplayStatics.GetPlayerCharacter` 0)))
  (bind _statscomp (`/Game/Player/BP_MagicianPlayerCharacter.StatsComp` _asbp_magician_player_character))
  (set `/Game/Blueprints/BP_StatsComponent.CurrentHealth` (`/Game/Blueprints/BP_StatsComponent.MaxHealth` _statscomp) _statscomp)
  (set `/Game/Blueprints/BP_StatsComponent.CurrentHealth` (`/Game/Blueprints/BP_StatsComponent.MaxHealth` _bp_statscomponent) _bp_statscomponent)
  (set `Widget.Visibility` "Collapsed" (`self.PlayerHUDRef`))
  (`KismetSystemLibrary.PrintString` "HUD Visable"))

(fn `SimpleAI`
  (params (timer :type "Float (double-precision)"))
  (returns (timerout :type "Float (double-precision)"))
  (if (`self.SimpleAiBool`)
    (set `self.Timer` (`self.InitialTImer`))
    (set `self.SimpleAiBool` false)
    (else
      (set `self.Timer` (/ (`self.InitialTImer`) 2.0))
      (set `self.SimpleAiBool` true)))
  (return (`self.Timer`)))

(fn `TimerEvent1`
  (bind _output_get (set `self.Timer` (`KismetMathLibrary.FClamp` (- (`self.Timer`) (`GameplayStatics.GetWorldDeltaSeconds`)) 0.0 (`self.Timer`))))
  (bind _asbp_magician_player_character (cast `/Game/Player/BP_MagicianPlayerCharacter` (`GameplayStatics.GetPlayerCharacter` 0)))
  (`/Game/Blueprints/BP_StatsComponent.TimerON` (`/Game/Player/BP_MagicianPlayerCharacter.StatsComp` _asbp_magician_player_character) _output_get))

(fn `UserConstructionScript`)

(fn `WaterEffect`
  (bind _returnvalue (`|SpawnActorFromClass` "/Game/SFX/Effects/Beams/BP_Waterbeam.BP_Waterbeam_C" (`KismetMathLibrary.Conv_VectorToTransform` (`SceneComponent.K2_GetComponentLocation` (`/Game/Blueprints/BP_Enemy.AtkAnimPos` (`self.Enemy1`)))) "Undefined" "MultiplyWithRoot" self null))
  (bind _returnvalue_2 (`self.GetTargetRotation`))
  (`SceneComponent.K2_SetWorldRotation` (`/Game/SFX/Effects/Beams/BP_Waterbeam.DefaultSceneRoot` _returnvalue) _returnvalue_2 false false)
  (`|SpawnActorFromClass` "/Game/SFX/Effects/Damage/BP_Damage_FX.BP_Damage_FX_C" (`KismetMathLibrary.Conv_VectorToTransform` (`SceneComponent.K2_GetComponentLocation` (`Character.Mesh` (`self.Enemy1`)))) "Undefined" "MultiplyWithRoot" null null))