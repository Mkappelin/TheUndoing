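; BP_Enemy is an enemy actor that hands off to BP_CombatHandler when the player character overlaps its sphere.
; It finds the handler on BeginPlay and passes itself through EnemyCollided on contact.
; TakeDamage and Spellaccuracy forward hit and spell results to the widget component for display.
; TakeDamage, OnAttack and Death set animation or state flags, with no health logic here; GetStatComponent is an empty stub.
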(event `self.ReceiveBeginPlay`
  (bind _returnvalue (`GameplayStatics.GetActorOfClass` "/Game/Blueprints/BP_CombatHandler.BP_CombatHandler_C"))
  (set `self.Combat handler` _returnvalue))

(event `self.Sphere1.OnComponentBeginOverlap`
  (params (OverlappedComponent :type "PrimitiveComponent Object Reference") (OtherActor :type "Actor Object Reference") (OtherComp :type "PrimitiveComponent Object Reference") (OtherBodyIndex :type Integer) (bFromSweep :type Boolean) (SweepResult :type "HitResult Structure (by ref)"))
  (if (== OtherActor (`GameplayStatics.GetPlayerCharacter` 0))
    (bind _asbp_combat_handler (cast `/Game/Blueprints/BP_CombatHandler` (`self.Combat handler`)))
    (`/Game/Blueprints/BP_CombatHandler.EnemyCollided` _asbp_combat_handler self 0.0 0 0.0)))

(fn `Death`
  (set `self.Deathbool` true))

(fn `GetStatComponent`
  (params (Statcomp :type "ActorComponent Object Reference")))

(fn `NewFunction`)

(fn `OnAttack`
  (set `self.AttackAnim` true))

(fn `Spellaccuracy`
  (params (`Failed combo` :type Boolean) (Damage :type "Float (double-precision)") (Spelltype :type "/Game/Blueprints/Spells Enum" :default "NewEnumerator0"))
  (message `/Game/UI/Widgets/BPI_DamNumbers.AccuracyWidgetHolder` (`WidgetComponent.GetUserWidgetObject` (`self.Widget`)) `Failed combo` Damage Spelltype))

(fn `TakeDamage`
  (params (Crit :type Boolean) (Damage :type "Float (double-precision)") (Spelltype :type "/Game/Blueprints/Spells Enum" :default "NewEnumerator0"))
  (message `/Game/UI/Widgets/BPI_DamNumbers.DamageNumbersWidgetFolder` (`WidgetComponent.GetUserWidgetObject` (`self.Widget`)) Crit Damage Spelltype)
  (set `self.TakeDmgAnim` true))

(fn `UserConstructionScript`)