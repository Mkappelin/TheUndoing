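; BP_EnemyChild is an enemy Blueprint that reports contact with the player to the combat handler.
; On BeginPlay it runs the parent logic, then finds and stores the BP_CombatHandler actor in the level.
; When the player character begins overlapping Sphere1, it calls EnemyCollided on that handler, passing itself with a fixed AI type and damage value.
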(event `self.ReceiveBeginPlay`
  (`parent.ReceiveBeginPlay`)
  (bind _returnvalue (`GameplayStatics.GetActorOfClass` "/Game/Blueprints/BP_CombatHandler.BP_CombatHandler_C"))
  (set `self.Combat handler` _returnvalue))

(event `self.Sphere1.OnComponentBeginOverlap`
  (params (OverlappedComponent :type "PrimitiveComponent Object Reference") (OtherActor :type "Actor Object Reference") (OtherComp :type "PrimitiveComponent Object Reference") (OtherBodyIndex :type Integer) (bFromSweep :type Boolean) (SweepResult :type "HitResult Structure (by ref)"))
  (if (== OtherActor (`GameplayStatics.GetPlayerCharacter` 0))
    (bind _asbp_combat_handler (cast `/Game/Blueprints/BP_CombatHandler` (`self.Combat handler`)))
    (`/Game/Blueprints/BP_CombatHandler.EnemyCollided` _asbp_combat_handler self 0.0 1 10.0)))

(fn `UserConstructionScript`
  (`parent.UserConstructionScript`))