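; Quest event trigger where the player solves a world obstacle by drawing a spell.
; Entering the sphere while active registers the event with the magician player, enters paint mode, and snaps the player to face a target.
; Recognized spells matching the solution are cast at that target; PlayEventFromSpell dispatches the type-specific effect, such as burning, lifting or repairing.
; CompleteEvent advances dialogue, exits paint mode, activates the next quest and destroys the actor.
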(event `self.Sphere1.OnComponentBeginOverlap`
  (params (OverlappedComponent :type "PrimitiveComponent Object Reference") (OtherActor :type "Actor Object Reference") (OtherComp :type "PrimitiveComponent Object Reference") (OtherBodyIndex :type Integer) (bFromSweep :type Boolean) (SweepResult :type "HitResult Structure (by ref)"))
  (bind _returnvalue (`GameplayStatics.GetPlayerCharacter` 0))
  (bind _returnvalue_2 (`GameplayStatics.GetPlayerCharacter` 0))
  (bind _returnvalue_3 (`SceneComponent.K2_GetComponentLocation` (`self.PlayerPos`)))
  ;[0 0.7656 0.02564 0.5] Lets Fix this
  (if (`self.Active`)
    (if (== OtherActor _returnvalue)
      (bind _asbp_magician_player_character (cast `/Game/Player/BP_MagicianPlayerCharacter` _returnvalue))
      (bind _output_get (set `self.Player` _asbp_magician_player_character))
      (`/Game/Player/BP_MagicianPlayerCharacter.BindActiveEvent` _output_get self)
      (bind _asbp_magician_player_controller (cast `/Game/Player/BP_MagicianPlayerController` (`GameplayStatics.GetPlayerController` 0)))
      (`MagicianPlayerController.EnterPaintMode` _asbp_magician_player_controller (`ActorComponent.GetOwner` (`self.Camera`)) 0.5)
      (add `MagicianPlayerController.OnSpellRecognized` _asbp_magician_player_controller (`|CreateDelegate` :!event `OnSpell`))
      (`self.K2_TeleportTo` :`self` _returnvalue :`DestLocation` _returnvalue_3)
      (`SceneComponent.K2_SetWorldRotation` (`Character.CapsuleComponent` _returnvalue_2) (`KismetMathLibrary.MakeRotator` 0.0 0.0 (.yaw (`KismetMathLibrary.FindLookAtRotation` _returnvalue_3 (`SceneComponent.K2_GetComponentLocation` (`Actor.RootComponent` (`|GetArrayItem` (`self.TargetActor`) (`KismetMathLibrary.FTrunc` (`self.TargetIndex`)))))))) false false)
      (`MovementComponent.StopMovementImmediately` (`Character.CharacterMovement` _returnvalue_2)))))

(event `OnSpell`
  (params (Result :type "SpellRecognitionResult Structure (by ref)"))
  (switch `string` (`.Name` (break `SpellRecognitionResult` Result))
    (:`Water`
      (set `self.Recognized Spell` "NewEnumerator0"))
    (:`Fire`
      (set `self.Recognized Spell` "NewEnumerator1"))
    (:`Lightning`
      (set `self.Recognized Spell` "NewEnumerator2"))
    (:`Lifting`
      (set `self.Recognized Spell` "NewEnumerator4"))
    (:`Wind`
      (set `self.Recognized Spell` "NewEnumerator5")))
  (if (`KismetArrayLibrary.Array_Contains` (`self.Event Solution Spell`) (`self.Recognized Spell`))
    (`self.BindEffectToSpell`)))

(event `CompleteEvent`
  (bind _speechref (`self.SpeechRef`))
  (set `self.EventComplete` true)
  (if (`KismetSystemLibrary.IsValid` _speechref)
    (`/Game/SpeechBubble/BP_SpeechActor.ProgressDialouge` _speechref))
  (`KismetSystemLibrary.Delay` 1.0)
  (bind _asbp_magician_player_controller (cast `/Game/Player/BP_MagicianPlayerController` (`GameplayStatics.GetPlayerController` 0)))
  (`MagicianPlayerController.ExitPaintMode` _asbp_magician_player_controller 0.5)
  (`self.ActivateNextQuest`)
  (`self.K2_DestroyActor`))

(event `BurnBush`
  (bind _returnvalue (`GameplayStatics.GetActorOfClass` "/Game/SFX/Effects/BurnEffect/BurnObject.BurnObject_C"))
  (`/Game/SFX/Effects/BurnEffect/BurnObject.Burn` _returnvalue))

(event `LightFirePit`
  (bind _returnvalue (`GameplayStatics.GetActorOfClass` "/Game/SFX/Effects/FirePit/Event_CampFire.Event_CampFire_C"))
  (`/Game/SFX/Effects/FirePit/Event_CampFire.LightFire` _returnvalue))

(event `ScareMothsAway`
  (bind _returnvalue (`GameplayStatics.GetActorOfClass` "/Game/SFX/Effects/LanternEvent/Lantern.Lantern_C"))
  (`/Game/SFX/Effects/LanternEvent/Lantern.ScareMoths` _returnvalue))

(event `LiftLog`
  (bind _returnvalue (`GameplayStatics.GetActorOfClass` "/Game/SFX/Effects/Lifting/LogEvent.LogEvent_C"))
  (`/Game/SFX/Effects/Lifting/LogEvent.LiftLog` _returnvalue)
  (`KismetSystemLibrary.Delay` 1.0)
  (bind _returnvalue_2 (`GameplayStatics.GetActorOfClass` "/Game/SFX/Effects/Lifting/LogEvent.LogEvent_C"))
  (`/Game/SFX/Effects/Lifting/LogEvent.StopLift` _returnvalue_2))

(event `Bridge`
  (bind _returnvalue (`GameplayStatics.GetActorOfClass` "/Game/SFX/Effects/Repair/BridgeEvent.BridgeEvent_C"))
  (`/Game/SFX/Effects/Repair/BridgeEvent.RepairBridge` _returnvalue))

(event `BreachGate`
  (bind _returnvalue (`GameplayStatics.GetActorOfClass` "/Game/SFX/Effects/Gate/BP_GateEvent.BP_GateEvent_C"))
  (`/Game/SFX/Effects/Gate/BP_GateEvent.Breach` _returnvalue))

(fn `ActivateNextQuest`
  (bind _nextquest (`self.NextQuest`))
  (if (`KismetSystemLibrary.IsValid` _nextquest)
    (set `/Game/Blueprints/BP_TestEvent.Active` true _nextquest)))

(fn `BindEffectToSpell`
  (set `self.ArrayLenght` (`KismetMathLibrary.Conv_IntToDouble` (`KismetArrayLibrary.Array_Length` (`self.TargetActor`))))
  (if (> (`self.ArrayLenght`) 0.0)
    (`/Game/Player/BP_MagicianPlayerCharacter.CastSpell` (`self.Player`) (`SceneComponent.K2_GetComponentLocation` (`Actor.RootComponent` (`|GetArrayItem` (`self.TargetActor`) (`KismetMathLibrary.FTrunc` (`self.TargetIndex`))))) (`self.Recognized Spell`) false)))

(fn `BindEnemy1`
  (params (Enemy :type "/Game/Blueprints/BP_Enemy Object Reference"))
  (set `self.Enemy` Enemy))

(fn `PlayEventFromSpell`
  (locals (NewLocalVar :type "/Game/SFX/Effects/Fire/FireEvent Object Reference"))
  (switch `/Game/Blueprints/Events` (`self.EventType`)
    (:`NewEnumerator1`
      (`self.BurnBush`))
    (:`NewEnumerator3`
      (`self.LiftLog`))
    (:`NewEnumerator2`
      (`self.LightFirePit`))
    (:`NewEnumerator4`
      (`self.ScareMothsAway`))
    (:`NewEnumerator5`
      (bind _asfire_event (cast `/Game/SFX/Effects/Fire/FireEvent` (`|GetArrayItem` (`self.TargetActor`) (`KismetMathLibrary.FTrunc` (`self.TargetIndex`)))))
      (`/Game/SFX/Effects/Fire/FireEvent.DestroyFire` _asfire_event))
    (:`NewEnumerator6`
      (`self.Bridge`))
    (:`NewEnumerator7`
      (`self.BreachGate`))))

(fn `UserConstructionScript`)