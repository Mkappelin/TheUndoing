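; BP_Player is the player Blueprint, set up as a test harness for stats, damage and the HUD.
; On BeginPlay it creates WBP_HUD and binds its own and the first found BP_Enemy's stats components to it, adding IMC_Test only if an enemy exists.
; IA_DamageEnemy applies fixed damage to that enemy type's stats component, while a raw 1 key, rather than the empty IA_DamagePlayer event, damages the player.
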(event `self.ReceiveBeginPlay`
  (bind _returnvalue (`|CreateWidget` "/Game/UI/Widgets/WBP_HUD.WBP_HUD_C" (`GameplayStatics.GetPlayerController` 0)))
  (set `self.HUDRef` _returnvalue)
  (set `/Game/UI/Widgets/WBP_HUD.PlayerStats` (`self.StatsComp`) (`self.HUDRef`))
  (bind _returnvalue_2 (`GameplayStatics.GetActorOfClass` "/Game/Blueprints/BP_Enemy.BP_Enemy_C"))
  (`/Engine/EditorBlueprintResources/StandardMacros.IsValid` _returnvalue_2
    (:`Is Valid`
      (set `/Game/UI/Widgets/WBP_HUD.EnemyStats` (`self.GetComponentByClass` _returnvalue_2 "/Game/Blueprints/BP_StatsComponent.BP_StatsComponent_C") (`self.HUDRef`))
      (`UserWidget.AddToViewport` (`self.HUDRef`) 0)
      (`KismetSystemLibrary.PrintString` "HUD Created")
      (`EnhancedInputSubsystemInterface.AddMappingContext` (pcsubsystem `EnhancedInputLocalPlayerSubsystem` (`GameplayStatics.GetPlayerController` 0)) "/Game/SpellDrawing/Player/Input/IMC_Test.IMC_Test" 0 (struct))
      (`KismetSystemLibrary.PrintString` "IMC Added" true true (struct :`R` 0.015711 :`G` 0.494792 :`B` 0.001651 :`A` 1.0)))
    (:`Is Not Valid`
      (`KismetSystemLibrary.PrintString` "BP_Player_No Enemy Found" true true (struct :`R` 0.463542 :`G` 0.022485 :`A` 1.0) 5.0)
      (`UserWidget.AddToViewport` (`self.HUDRef`) 0))))

(event `EnhancedInput|/Game/SpellDrawing/Player/Input/IA_DamageEnemy`
  (params (ActionValue :type Boolean) (ElapsedSeconds :type "Float (double-precision)") (TriggeredSeconds :type "Float (double-precision)") (InputAction :type "InputAction Object Reference" :default "/Game/SpellDrawing/Player/Input/IA_DamageEnemy.IA_DamageEnemy"))
  (:`Started`
    (`KismetSystemLibrary.PrintString` "Enemy IA Started")
    (bind _returnvalue (`GameplayStatics.GetActorOfClass` "/Game/Blueprints/BP_Enemy.BP_Enemy_C"))
    (bind _returnvalue_2 (`self.GetComponentByClass` _returnvalue "/Game/Blueprints/BP_StatsComponent.BP_StatsComponent_C"))
    (`/Engine/EditorBlueprintResources/StandardMacros.IsValid` _returnvalue_2
      (:`Is Valid`
        (`/Game/Blueprints/BP_StatsComponent.TakeDamageSimple` _returnvalue_2 10.0))
      (:`Is Not Valid`
        (`KismetSystemLibrary.PrintString` "BP_Player_EnemyNotFound" true true (struct :`R` 0.385417 :`G` 0.023661 :`A` 1.0) 5.0)))))

(event `EnhancedInput|/Game/SpellDrawing/Player/Input/IA_DamagePlayer`
  (params (ActionValue :type Boolean) (ElapsedSeconds :type "Float (double-precision)") (TriggeredSeconds :type "Float (double-precision)") (InputAction :type "InputAction Object Reference" :default "/Game/SpellDrawing/Player/Input/IA_DamagePlayer.IA_DamagePlayer")))

(event `Key|One`
  (params (Key :type "Key Structure"))
  (:`Pressed`
    (`KismetSystemLibrary.PrintString` "Player IA Started")
    (`/Game/Blueprints/BP_StatsComponent.TakeDamageSimple` (`self.StatsComp`) 10.0)))

(fn `UserConstructionScript`)