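; Stats component that tracks an owner's health and a combat countdown timer.
; Simple damage lowers current health within zero and max, and a getter returns it as a clamped fraction.
; StartCombatTimer activates a Tick-driven countdown that refills to its duration and keeps looping at zero.
; TimerON overrides the remaining time without activating it, and GetTimerPercent caps its ratio at the remaining time rather than one.
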(event `StartCombatTimer`
  (params (Duration :type "Float (double-precision)" :default 15.0))
  (bind _output_get (set `self.CombatTimerDuration` Duration))
  (set `self.CombatTimerRemaining` _output_get)
  (set `self.CombatTimerActive` true))

(event `self.ReceiveTick`
  (params (DeltaSeconds :type "Float (single-precision)"))
  (if (`self.CombatTimerActive`)
    (bind _output_get (set `self.CombatTimerRemaining` (`KismetMathLibrary.FClamp` (- (`self.CombatTimerRemaining`) DeltaSeconds) 0.0 (`self.CombatTimerDuration`))))
    (if (<= _output_get 0.0)
      (set `self.CombatTimerActive` true)
      (set `self.CombatTimerRemaining` (`self.CombatTimerDuration`)))))

(fn `GetHealthPercent`
  (returns (Percent :type "Float (double-precision)"))
  (bind _maxhealth (`self.MaxHealth`))
  (return (`KismetMathLibrary.FClamp` (`KismetMathLibrary.SelectFloat` 0.0 (/ (`self.CurrentHealth`) _maxhealth) (<= _maxhealth 0.0)))))

(fn `GetTimerPercent`
  (returns (Percent :type "Float (double-precision)"))
  (bind _combattimerremaining (`self.CombatTimerRemaining`))
  (return (`KismetMathLibrary.FClamp` (/ _combattimerremaining (`self.CombatTimerDuration`)) 0.0 _combattimerremaining)))

(fn `TakeDamageSimple`
  (params (Amount :type "Float (double-precision)"))
  (if (> Amount 0.0)
    (set `self.CurrentHealth` (`KismetMathLibrary.FClamp` (- (`self.CurrentHealth`) Amount) 0.0 (`self.MaxHealth`)))))

(fn `TimerON`
  (params (Amount :type "Float (double-precision)"))
  (if (> Amount 0.0)
    (set `self.CombatTimerRemaining` (`KismetMathLibrary.FClamp` Amount 0.0 (`self.CombatTimerDuration`)))))