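; SpellEventActor is a trigger actor that teleports the player when they enter its sphere volume.
; When Sphere1 overlaps the player character, it moves them to the location and rotation of its PlayerPos component.
; The teleport runs only if the game mode is BP_MagicianGameModeBase; otherwise it prints a failure message.
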(event `self.Sphere1.OnComponentBeginOverlap`
  (params (OverlappedComponent :type "PrimitiveComponent Object Reference") (OtherActor :type "Actor Object Reference") (OtherComp :type "PrimitiveComponent Object Reference") (OtherBodyIndex :type Integer) (bFromSweep :type Boolean) (SweepResult :type "HitResult Structure (by ref)"))
  (bind _returnvalue (`GameplayStatics.GetPlayerCharacter` 0))
  (bind _playerpos (`self.PlayerPos`))
  (if (== OtherActor _returnvalue)
    (cast `/Game/Blueprints/BP_MagicianGameModeBase` (`GameplayStatics.GetGameMode`)
      (:`then`
        (`self.K2_TeleportTo` _returnvalue (`SceneComponent.K2_GetComponentLocation` _playerpos) (`SceneComponent.K2_GetComponentRotation` _playerpos)))
      (:`CastFailed`
        (`KismetSystemLibrary.PrintText` "Cast Failed")))))

(fn `UserConstructionScript`)