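; Boar enemy that chases the player and hands off to BP_CombatHandler on contact, extending a parent enemy class.
; One sphere overlap starts a Tick-driven, swept VInterpTo chase, while the other stops it and calls EnemyCollided with the boar's damage and AI settings.
; Parent overrides trigger attack and damage animations that return to idle after a shared delay.
; Death activates a smoke effect briefly, then destroys the actor.
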(event `self.ReceiveBeginPlay`
  (`parent.ReceiveBeginPlay`)
  (bind _returnvalue (`GameplayStatics.GetActorOfClass` "/Game/Blueprints/BP_CombatHandler.BP_CombatHandler_C"))
  (set `self.Combat handler` _returnvalue))

(event `self.ReceiveTick`
  (params (DeltaSeconds :type "Float (single-precision)"))
  (bind _returnvalue (`self.K2_GetActorLocation`))
  (bind _returnvalue_2 (`self.K2_GetActorLocation` (`GameplayStatics.GetPlayerCharacter` 0)))
  (`parent.ReceiveTick` DeltaSeconds)
  (if (`self.IsMoving`)
    (`self.K2_SetActorLocationAndRotation` (`KismetMathLibrary.VInterpTo` _returnvalue _returnvalue_2 DeltaSeconds 1.0) (`KismetMathLibrary.FindLookAtRotation` _returnvalue_2 _returnvalue) true)))

(event `self.Sphere1.OnComponentBeginOverlap`
  (params (OverlappedComponent :type "PrimitiveComponent Object Reference") (OtherActor :type "Actor Object Reference") (OtherComp :type "PrimitiveComponent Object Reference") (OtherBodyIndex :type Integer) (bFromSweep :type Boolean) (SweepResult :type "HitResult Structure (by ref)"))
  (if (== OtherActor (`GameplayStatics.GetPlayerCharacter` 0))
    (bind _asbp_combat_handler (cast `/Game/Blueprints/BP_CombatHandler` (`self.Combat handler`)))
    (set `self.IsMoving` false)
    (`/Game/Blueprints/BP_CombatHandler.EnemyCollided` _asbp_combat_handler self (`self.Timer`) (`self.AItype`) 8.0)))

(event `Attack`
  (bind _mesh (`self.Mesh`))
  (`SkeletalMeshComponent.PlayAnimation` _mesh "/Game/Assets/CampSite/Boar/EnemyBoarAttack_Anim.EnemyBoarAttack_Anim" false)
  (`KismetSystemLibrary.Delay` 0.6 :!label _label)
  (`SkeletalMeshComponent.PlayAnimation` _mesh "/Game/Assets/CampSite/Boar/BoarEnemy_idle.BoarEnemy_idle" true))

(event `self.Sphere2.OnComponentBeginOverlap`
  (params (OverlappedComponent :type "PrimitiveComponent Object Reference") (OtherActor :type "Actor Object Reference") (OtherComp :type "PrimitiveComponent Object Reference") (OtherBodyIndex :type Integer) (bFromSweep :type Boolean) (SweepResult :type "HitResult Structure (by ref)"))
  (if (== OtherActor (`GameplayStatics.GetPlayerCharacter` 0))
    (set `self.IsMoving` true)))

(event `TakeDamageAnim`
  (`SkeletalMeshComponent.PlayAnimation` (`self.Mesh`) "/Game/Assets/CampSite/Boar/EnemyBoarDamage.EnemyBoarDamage" false)
  (goto _label))

(event `BoarDeath`
  (`ActorComponent.Activate` (`self.RepairSmoke`) false)
  (`KismetSystemLibrary.Delay` 1.5)
  (`ActorComponent.Deactivate` (`self.RepairSmoke`))
  (`self.K2_DestroyActor`))

(fn `Death`
  (`parent.Death`)
  (`self.BoarDeath`))

(fn `OnAttack`
  (`parent.OnAttack`)
  (`self.Attack`))

(fn `SpellAccuracyFeedback`
  (params (Crit :type Boolean) (Accuracy :type "Float (double-precision)") (Spelltype :type "/Game/Blueprints/Spells Enum" :default "NewEnumerator0"))
  (`parent.SpellAccuracyFeedback` Crit Accuracy Spelltype))

(fn `TakeDamage`
  (params (Crit :type Boolean) (Damage :type "Float (double-precision)") (Spelltype :type "/Game/Blueprints/Spells Enum" :default "NewEnumerator0"))
  (`parent.TakeDamage` Crit Damage Spelltype)
  (`self.TakeDamageAnim`))

(fn `UserConstructionScript`
  (`parent.UserConstructionScript`))