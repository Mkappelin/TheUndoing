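; Test enemy that runs a spell-drawing battle when the player overlaps its trigger sphere.
; Overlap teleports the player to a set spot, switches the magician controller into paint mode and binds recognized spells.
; Circle, X and Star deal score-scaled damage, while Triangle raises a temporary block halving enemy hits.
; Tick drives the block and attack countdowns; enemy death exits paint mode and destroys the actor.
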(event `self.ReceiveTick`
  (params (DeltaSeconds :type "Float (single-precision)"))
  (if (`self.InCombat`)
    (`self.TimerEvent`)
    (if (`self.IsBlock`)
      (`self.BlockTImerEvent`))
    (if (== (`self.Timer`) 0.0)
      (`self.EnemyAttack`))
    (`KismetSystemLibrary.Delay` 1.0)
    (`KismetSystemLibrary.PrintString` (`KismetStringLibrary.Conv_DoubleToString` (`self.BlockTimer`)))))

(event `self.Sphere1.OnComponentBeginOverlap`
  (params (OverlappedComponent :type "PrimitiveComponent Object Reference") (OtherActor :type "Actor Object Reference") (OtherComp :type "PrimitiveComponent Object Reference") (OtherBodyIndex :type Integer) (bFromSweep :type Boolean) (SweepResult :type "HitResult Structure (by ref)"))
  (bind _returnvalue (`GameplayStatics.GetPlayerCharacter` 0))
  (bind _returnvalue_2 (`SceneComponent.K2_GetComponentLocation` (`self.PlayerPos`)))
  (if (== OtherActor _returnvalue)
    (bind _asbp_magician_player_controller (cast `/Game/Blueprints/BP_MagicianPlayerController` (`GameplayStatics.GetPlayerController` 0)))
    (`MagicianPlayerController.EnterPaintMode` _asbp_magician_player_controller (`ActorComponent.GetOwner` (`self.Camera`)) 0.5)
    (add `MagicianPlayerController.OnSpellRecognized` _asbp_magician_player_controller (`|CreateDelegate` :!event `OnSpell`))
    (`self.K2_TeleportTo` :`self` _returnvalue :`DestLocation` _returnvalue_2)
    (`Controller.SetControlRotation` (`GameplayStatics.GetPlayerController` 0) (`KismetMathLibrary.FindLookAtRotation` _returnvalue_2 (`self.K2_GetActorLocation` self)))
    (`self.BattleBegin`)))

(event `BlockTImerEvent`
  (bind _output_get (set `self.BlockTimer` (`KismetMathLibrary.FClamp` (- (`self.BlockTimer`) (stale `self.ReceiveTick` DeltaSeconds)) 0.0 (`self.BlockTimer`))))
  (if (== _output_get 0.0)
    (set `self.IsBlock` false)
    (set `self.BlockTimer` 5.0)))

(event `PlayerBlock`
  (set `self.IsBlock` true)
  (`KismetSystemLibrary.PrintString` (`KismetStringLibrary.Conv_BoolToString` (`self.IsBlock`))))

(event `OnSpell`
  (params (Result :type "SpellRecognitionResult Structure (by ref)"))
  (bind (_bsuccess _name _score) (break `SpellRecognitionResult` Result))
  (set `self.PlayerDMG` (`KismetMathLibrary.Round` (* _score (`KismetMathLibrary.Conv_IntToDouble` (`self.PlayerDMGOriginal`)))))
  (`KismetSystemLibrary.PrintString` (`KismetStringLibrary.Concat_StrStr` "Spell Success: " (`KismetStringLibrary.Conv_BoolToString` _bsuccess) ", Shape: " _name ", Score: " (`KismetStringLibrary.Conv_DoubleToString` _score)) true true (struct :`G` 0.66 :`B` 1.0 :`A` 1.0) 5.0)
  (if (== _name "Circle")
    (`self.PlayerAttack`)
    (elif (== _name "Triangle")
      (`self.PlayerBlock`)
      (elif (== _name "X")
        (`self.PlayerAttack`)
        (elif (== _name "Star")
          (`self.PlayerAttack`))))))

(event `PlayerAttack`
  (bind _enemyhp (`self.EnemyHP`))
  (if (`self.PlayerTurn`)
    (bind _asbp_magician_player_controller (cast `/Game/Blueprints/BP_MagicianPlayerController` (`GameplayStatics.GetPlayerController` 0)))
    (set `MagicianPlayerController.bIsPaintingMode` false _asbp_magician_player_controller)
    (`KismetSystemLibrary.Delay` 1.0)
    (set `self.EnemyHP` (- (`self.EnemyHP`) (`self.PlayerDMG`)))
    (set `MagicianPlayerController.bIsPaintingMode` true _asbp_magician_player_controller)
    (`KismetSystemLibrary.PrintString` (`KismetStringLibrary.Concat_StrStr` "Enemy HP:" (`KismetStringLibrary.Conv_IntToString` _enemyhp)))
    (if (<= _enemyhp 0)
      (`self.EnemyDeath`))))

(event `BattleBegin`
  (set `self.IsBlock` false)
  (set `self.PlayerTurn` true)
  (set `self.Timer` 10.0)
  (set `self.InCombat` true)
  (set `self.BlockTimer` 5.0))

(event `EnemyDeath`
  (bind _asbp_magician_player_controller (cast `/Game/Blueprints/BP_MagicianPlayerController` (`GameplayStatics.GetPlayerController` 0)))
  (set `MagicianPlayerController.bIsPaintingMode` true _asbp_magician_player_controller)
  (`MagicianPlayerController.ExitPaintMode` _asbp_magician_player_controller 0.5)
  (`self.K2_DestroyActor`))

(event `TimerEvent`
  (set `self.Timer` (`KismetMathLibrary.FClamp` (- (`self.Timer`) (`GameplayStatics.GetWorldDeltaSeconds`)) 0.0 (`self.Timer`))))

(event `EnemyAttack`
  (bind _returnvalue (`GameplayStatics.GetPlayerController` 0))
  (bind _asbp_magician_player_controller (cast `/Game/Blueprints/BP_MagicianPlayerController` _returnvalue))
  (set `MagicianPlayerController.bIsPaintingMode` false _asbp_magician_player_controller)
  (if (`self.IsBlock`)
    (set `self.Player_HP` (- (`self.Player_HP`) (/ (`self.EnemyDMG`) 2)))
    (else
      (set `self.Player_HP` (- (`self.Player_HP`) (`self.EnemyDMG`)))))
  (set `self.InCombat` false)
  (set `self.Timer` 10.0)
  (`KismetSystemLibrary.Delay` 2.0)
  (set `self.InCombat` true)
  (`KismetSystemLibrary.PrintString` (`KismetStringLibrary.Concat_StrStr` "Player HP:" (`KismetStringLibrary.Conv_IntToString` (`self.Player_HP`))))
  (bind _asbp_magician_player_controller_2 (cast `/Game/Blueprints/BP_MagicianPlayerController` _returnvalue))
  (set `MagicianPlayerController.bIsPaintingMode` true _asbp_magician_player_controller_2))

(fn `UserConstructionScript`)