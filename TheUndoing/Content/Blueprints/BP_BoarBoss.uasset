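; Boar boss character that starts a combat encounter on player overlap and turns into a rescued-brother dialogue moment on death.
; Sphere overlap flags the AnimBP as in combat and registers the boss with BP_CombatHandler, found at BeginPlay.
; Tick polls boolean flags to play a random attack montage, a damage montage, or death.
; Death plays smoke, spawns BP_BrotherGuy and a dialogue actor using DT_BrotherBoar, then destroys the boss.
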(event `self.ReceiveBeginPlay`
  (`parent.ReceiveBeginPlay`)
  (bind _returnvalue (`GameplayStatics.GetActorOfClass` "/Game/Blueprints/BP_CombatHandler.BP_CombatHandler_C"))
  (set `self.Combat handler` _returnvalue))

(event `self.ReceiveTick`
  (params (DeltaSeconds :type "Float (single-precision)"))
  (`parent.ReceiveTick` DeltaSeconds)
  (if (`self.Deathbool`)
    (`self.BossDeath`)
    (elif (`self.AttackAnim`)
      (`self.Attack`)
      (elif (`self.TakeDmgAnim`)
        (`self.TakeDamageAnim`)))))

(event `BossDeath`
  (bind _returnvalue (`self.GetTransform`))
  (`ActorComponent.Activate` (`self.RepairSmoke`) false)
  (`KismetSystemLibrary.Delay` 1.0)
  (`ActorComponent.Deactivate` (`self.RepairSmoke`))
  (`|SpawnActorFromClass` "/Game/Characters/BP_BrotherGuy.BP_BrotherGuy_C" _returnvalue "Undefined" "MultiplyWithRoot" null null)
  (`|SpawnActorFromClass` "/Game/SpeechBubble/BP_SpeechActor.BP_SpeechActor_C" _returnvalue "Undefined" "MultiplyWithRoot" null "/Game/SpeechBubble/Dialouges/DT_BrotherBoar.DT_BrotherBoar" null)
  (set `self.Deathbool` false)
  (`self.K2_DestroyActor`))

(event `self.Sphere1.OnComponentBeginOverlap`
  (params (OverlappedComponent :type "PrimitiveComponent Object Reference") (OtherActor :type "Actor Object Reference") (OtherComp :type "PrimitiveComponent Object Reference") (OtherBodyIndex :type Integer) (bFromSweep :type Boolean) (SweepResult :type "HitResult Structure (by ref)"))
  (if (== OtherActor (`GameplayStatics.GetPlayerCharacter` 0))
    (bind _asabp_boar_boss (cast `/Game/Assets/CampSite/Boar/BoarBoss/ABP_BoarBoss` (`SkeletalMeshComponent.GetAnimInstance` (`self.Mesh`))))
    (set `/Game/Assets/CampSite/Boar/BoarBoss/ABP_BoarBoss.InCombat` true _asabp_boar_boss)
    (bind _asbp_combat_handler (cast `/Game/Blueprints/BP_CombatHandler` (`self.Combat handler`)))
    (`/Game/Blueprints/BP_CombatHandler.EnemyCollided` _asbp_combat_handler self 0.0 1 8.0)))

(event `Attack`
  (set `self.AttackAnim` false)
  (if (`KismetMathLibrary.RandomBool`)
    (`self.PlayAnimMontage` "/Game/Assets/CampSite/Boar/BoarBoss/BossAttack2.BossAttack2" 1.8)
    (else
      (`self.PlayAnimMontage` "/Game/Assets/CampSite/Boar/BoarBoss/BossAttack1.BossAttack1" 1.3 "Default"))))

(event `TakeDamageAnim`
  (set `self.TakeDmgAnim` false)
  (`self.PlayAnimMontage` "/Game/Assets/CampSite/Boar/BoarBoss/BossTakeDamage.BossTakeDamage" 1.5))

(fn `UserConstructionScript`
  (`parent.UserConstructionScript`))