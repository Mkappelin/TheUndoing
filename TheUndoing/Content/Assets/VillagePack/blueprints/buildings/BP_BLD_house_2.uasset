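; Village house Blueprint with four fire components that are put out through an Extinguish event.
; Each call picks a fire in reverse array order using FireIndex and shrinks it with the FadeFire timeline.
; When the timeline finishes, it hides and destroys that fire and increments the index.
; Once the index reaches five, a short delay precedes calling CompleteEvent on the referenced Event.
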(event `Extinguish`
  (bind _array (`|MakeArray` (`self.FIRE_1`) (`self.FIRE_2`) (`self.FIRE_3`) (`self.FIRE_4`)))
  (bind _returnvalue (`KismetArrayLibrary.Array_Length` _array))
  (if (> _returnvalue 0)
    (set `self.Current fire` (`|GetArrayItem` _array (`KismetMathLibrary.FTrunc` (- _returnvalue (`self.FireIndex`)))))
    (bind (_direction _shrinkfire) (`Timeline|FadeFire` :!via `PlayFromStart`)
      (:`Update`
        (`SceneComponent.SetRelativeScale3D` (`self.Current fire`) (`KismetMathLibrary.Conv_DoubleToVector` _shrinkfire)))
      (:`Finished`
        (`SceneComponent.SetHiddenInGame` (`self.Current fire`) true true)
        (`ActorComponent.K2_DestroyComponent` (`self.Current fire`))
        (set `self.FireIndex` (+ (`self.FireIndex`) 1.0))
        (if (== (`self.FireIndex`) 5.0)
          (`KismetSystemLibrary.Delay` 1.0)
          (`/Game/Blueprints/BP_TestEvent.CompleteEvent` (`self.Event`)))))))

(fn `UserConstructionScript`)