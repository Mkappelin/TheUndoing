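; Player magician character that casts elemental spells from a staff and owns the player HUD.
; CastSpell stores spell type and target and plays the cast montage; SpawnSpellProjectile spawns the matching water, fire, lightning or force orb at the staff socket, aimed at the target.
; BeginPlay creates the HUD with player stats, and EnemyOverlap shows it, binding enemy stats and adding input mapping for valid enemies.
; Key 2 restores full health.
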(event `self.ReceiveBeginPlay`
  (bind _returnvalue (`|CreateWidget` "/Game/UI/Widgets/WBP_HUD.WBP_HUD_C" (`GameplayStatics.GetPlayerController` 0)))
  (set `self.HUDRef` _returnvalue)
  (set `/Game/UI/Widgets/WBP_HUD.PlayerStats` (`self.StatsComp`) (`self.HUDRef`)))

(event `Key|Two`
  (params (Key :type "Key Structure"))
  (bind _statscomp (`self.StatsComp`))
  (:`Pressed`
    (set `/Game/Blueprints/BP_StatsComponent.CurrentHealth` (`/Game/Blueprints/BP_StatsComponent.MaxHealth` _statscomp) _statscomp)))

(event `EnemyOverlap`
  (params (NewParam :type "/Game/Blueprints/BP_Enemy Object Reference"))
  (`/Engine/EditorBlueprintResources/StandardMacros.IsValid` NewParam
    (:`Is Valid`
      (set `/Game/UI/Widgets/WBP_HUD.EnemyStats` (`self.GetComponentByClass` NewParam "/Game/Blueprints/BP_StatsComponent.BP_StatsComponent_C") (`self.HUDRef`))
      (`UserWidget.AddToViewport` (`self.HUDRef`) 0)
      (`KismetSystemLibrary.PrintString` "HUD Created")
      (`EnhancedInputSubsystemInterface.AddMappingContext` (pcsubsystem `EnhancedInputLocalPlayerSubsystem` (`GameplayStatics.GetPlayerController` 0)) null 0 (struct))
      (`KismetSystemLibrary.PrintString` "IMC Added" true true (struct :`R` 0.015711 :`G` 0.494792 :`B` 0.001651 :`A` 1.0)))
    (:`Is Not Valid`
      (`KismetSystemLibrary.PrintString` "BP_Player_No Enemy Found" true true (struct :`R` 0.463542 :`G` 0.022485 :`A` 1.0) 5.0)
      (`UserWidget.AddToViewport` (`self.HUDRef`) 0))))

(fn `BindActiveEvent`
  (params (CurrentEvent :type "/Game/Blueprints/Events/BP_EventMaster Object Reference"))
  (set `self.ActiveEvent` CurrentEvent))

(fn `CastSpell`
  (params (Target :type "Vector Structure") (SpellType :type "/Game/Blueprints/Spells Enum" :default "NewEnumerator0"))
  (set `self.Spell Type` SpellType)
  (set `self.SpellTarget` Target)
  (bind _asbp_magician_player_character (cast `/Game/Player/BP_MagicianPlayerCharacter` (`GameplayStatics.GetPlayerCharacter` 0)))
  (`self.PlayAnimMontage` _asbp_magician_player_character "/Game/Player/Animations/CastSequence.CastSequence" 2.0 "None"))

(fn `SpawnSpellProjectile`
  (bind _returnvalue (`SceneComponent.GetSocketLocation` (`self.Staff_fbx_PROP_Staff`) "Staffend"))
  (bind _returnvalue_2 (`KismetMathLibrary.MakeTransform` _returnvalue (`KismetMathLibrary.FindLookAtRotation` _returnvalue (`self.SpellTarget`))))
  (`GameplayStatics.PlaySound2D` "/Game/Sounds/FireCast.FireCast" 0.5 1.0 0.0 null null)
  (switch `/Game/Blueprints/Spells` (`self.Spell Type`)
    (:`NewEnumerator0`
      (`|SpawnActorFromClass` "/Game/SFX/Effects/Orbs/BP_WaterOrb.BP_WaterOrb_C" _returnvalue_2 "Undefined" "MultiplyWithRoot" null null))
    (:`NewEnumerator1`
      (`|SpawnActorFromClass` "/Game/SFX/Effects/Orbs/BP_Fireball.BP_Fireball_C" _returnvalue_2 "Undefined" "MultiplyWithRoot" null null))
    (:`NewEnumerator2`
      (`|SpawnActorFromClass` "/Game/SFX/Effects/Orbs/BP_LightningOrb.BP_LightningOrb_C" _returnvalue_2 "Undefined" "MultiplyWithRoot" null null))
    (:`NewEnumerator4`
      (`|SpawnActorFromClass` "/Game/SFX/Effects/Orbs/BP_ForceOrb.BP_ForceOrb_C" _returnvalue_2 "Undefined" "MultiplyWithRoot" null null)))
  (return))

(fn `UserConstructionScript`)