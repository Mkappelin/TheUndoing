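; Player controller for the magician, handling movement, sprint, interaction, spellbook opening, combat combo input and spell painting.
; Enhanced Input drives camera-relative movement and paint events, while debug key T toggles paint mode and Q signals the CombatHandler.
; While painting, the deprojected mouse position moves a Niagara point effect and, for ribbon strokes, feeds a trail styled from the paint widget.
; Spaced stroke positions are recorded and burst into colored poofs with sound on release.
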(event Input|EnhancedActionEvents|EnhancedInputActionIA_Movement
  (params (ActionValue :type Vector%202D%20Structure) (ElapsedSeconds :type Float%20%28double-precision%29) (TriggeredSeconds :type Float%20%28double-precision%29) (InputAction :type Input%20Action%20Object%20Reference :default "/Game/Player/Input/IA_Movement.IA_Movement"))
  (bind _returnvalue (Game|GetPlayerCharacter 0))
  (bind (_x _y) (Math|Vector2D|BreakVector2D ActionValue))
  (bind _asbp_magician_player_character (Utilities|Casting|CastToBP_MagicianPlayerCharacter _returnvalue))
  (Pawn|Input|AddMovementInput _returnvalue (+ (* _y (Math|Vector|GetForwardVector (Class|SpringArmComponent|GetTargetRotation (Variables|/Game/Player/BP_MagicianPlayerCharacter.BP_MagicianPlayerCharacter_C|GetSpringArm _asbp_magician_player_character)))) (* _x (Math|Vector|GetRightVector (Class|SpringArmComponent|GetTargetRotation (Variables|/Game/Player/BP_MagicianPlayerCharacter.BP_MagicianPlayerCharacter_C|GetSpringArm _asbp_magician_player_character))) -1.0)) 1.0 false))

(event Input|EnhancedActionEvents|EnhancedInputActionIA_Sprint
  (params (ActionValue :type Boolean) (ElapsedSeconds :type Float%20%28double-precision%29) (TriggeredSeconds :type Float%20%28double-precision%29) (InputAction :type Input%20Action%20Object%20Reference :default "/Game/Player/Input/IA_Sprint.IA_Sprint"))
  (:Triggered
    (Variables|Default|SetMovementSpeed (Variables|Default|GetSprintSpeed))
    (Variables|/Script/Engine.CharacterMovementComponent|SetMaxWalkSpeed (Variables|/Script/Engine.Character|GetCharacterMovement (Game|GetPlayerCharacter 0)) (Variables|Default|GetMovementSpeed) :!label _label))
  (:Completed
    (Variables|Default|SetMovementSpeed (Variables|Default|GetWalkSpeed))
    (goto _label)))

(event Input|EnhancedActionEvents|EnhancedInputActionIA_Interact
  (params (ActionValue :type Boolean) (ElapsedSeconds :type Float%20%28double-precision%29) (TriggeredSeconds :type Float%20%28double-precision%29) (InputAction :type Input%20Action%20Object%20Reference :default "/Game/Player/Input/IA_Interact.IA_Interact"))
  (:Started
    (Default|CallOnTryInteract)))

(event Input|EnhancedActionEvents|EnhancedInputActionIA_PaintAction
  (params (ActionValue :type Boolean) (ElapsedSeconds :type Float%20%28double-precision%29) (TriggeredSeconds :type Float%20%28double-precision%29) (InputAction :type Input%20Action%20Object%20Reference :default "/Game/Player/Input/IA_PaintAction.IA_PaintAction"))
  (bind _bispaintingmode (Variables|Default|GetbIsPaintingMode))
  (:Triggered
    (Class|MagicianPlayerController|PressedtoPaint)
    (if _bispaintingmode
      (CallFunction|SpellDrawUpdate)))
  (:Started
    (if _bispaintingmode
      (Utilities|IsValid (Variables|Default|GetDrawTrailComponent)
        (:Is%20Valid
          _)
        (:Is%20Not%20Valid
          (CallFunction|SpellDrawSpawnComponents)))
      (CallFunction|SpellDrawSetActive true)))
  (:Completed
    (Class|MagicianPlayerController|ReleasedtoPaint)
    (if _bispaintingmode
      (CallFunction|SpellDrawSetActive false))))

(event Input|EnhancedActionEvents|EnhancedInputActionIA_MenuToggle
  (params (ActionValue :type Boolean) (ElapsedSeconds :type Float%20%28double-precision%29) (TriggeredSeconds :type Float%20%28double-precision%29) (InputAction :type Input%20Action%20Object%20Reference :default "/Game/Player/Input/IA_MenuToggle.IA_MenuToggle"))
  (:Started
    (bind _returnvalue (Actor|GetActorOfClass "/Game/UI/Systems/UIManager.UIManager_C"))
    (Default|OpenSpellbookUI _returnvalue)))

(event EventBeginPlay
  (Input|AddMappingContext (PlayerController|LocalPlayerSubsystems|GetEnhancedInputLocalPlayerSubsystem) "/Game/Player/Input/IMC_Magician.IMC_Magician" 0 "(bIgnoreAllPressedKeysUntilRelease=True,bForceImmediately=False,bNotifyUserSettings=False)")
  (bind _output_get (Variables|Default|SetMovementSpeed (Variables|Default|GetWalkSpeed)))
  (Variables|/Script/Engine.CharacterMovementComponent|SetMaxWalkSpeed (Variables|/Script/Engine.Character|GetCharacterMovement (Game|GetPlayerCharacter 0)) _output_get)
  (bind _returnvalue (Actor|GetActorOfClass "/Game/Blueprints/BP_CombatHandler.BP_CombatHandler_C"))
  (Variables|Default|SetCombatHandler _returnvalue))

(event EventTick
  (params (DeltaSeconds :type Float%20%28single-precision%29)))

(event Input|KeyboardEvents|DebugKeyT
  (params (Key :type Key%20Structure :default "None") (ActionValue :type Input%20Action%20Value%20Structure))
  (:Pressed
    (Class|MagicianPlayerController|TogglePaintMode)
    (Variables|Default|SetdebugMode (not (Variables|Default|GetbIsPaintingMode)))))

(event Input|KeyboardEvents|Q
  (params (Key :type Key%20Structure :default "None"))
  (bind _combathandler (Variables|Default|GetCombatHandler))
  (:Pressed
    (Default|ComboON _combathandler))
  (:Released
    (Default|ComboOFF _combathandler)))

(fn ConstructionScript)

(fn IsUsingRibbon
  (bind _returnvalue (Class|MagicianPlayerController|GetPaintWidget))
  (if (Utilities|IsValid _returnvalue)
    (return (Utilities|Enum|Equal(Enum) (Variables|/Script/TheUndoing.PaintWidget|GetStrokeType _returnvalue) "NiagaraRibbon"))
    (else
      (return false))))

(fn GetMouseonScreenPos
  (bind _returnvalue (Class|WidgetLayoutLibrary|GetMousePositiononViewport))
  (return (+ (.WorldPosition (Class|GameplayStatics|DeprojectScreentoWorld self (* _returnvalue (Class|WidgetLayoutLibrary|GetViewportScale)))) (* (.WorldDirection (Class|GameplayStatics|DeprojectScreentoWorld self (* _returnvalue (Class|WidgetLayoutLibrary|GetViewportScale)))) (Variables|Default|GetSpellDrawDistance)))))

(fn SpellDrawSpawnComponents
  (bind _returnvalue (Game|Player|GetPlayerPawn 0))
  (bind _returnvalue_2 (Class|MagicianPlayerController|GetPaintWidget))
  (bind _spelldrawscale (Variables|Default|GetSpellDrawScale))
  (bind _rootcomponent (Variables|/Script/Engine.Actor|GetRootComponent _returnvalue))
  (Utilities|FlowControl|Sequence
    (:then_0
      (bind _isusingribbon (CallFunction|IsUsingRibbon))
      (if _isusingribbon
        (bind _returnvalue_3 (Niagara|SpawnSystemAttached (Variables|Default|GetDrawTrailSystem) _rootcomponent "None" "0, 0, 0" "0, 0, 0" "KeepRelativeOffset" false false))
        (bind _output_get (Variables|Default|SetDrawTrailComponent _returnvalue_3))
        (Utilities|IsValid _output_get
          (:Is%20Valid
            (Effects|Components|ParticleSystem|SetColorParameter _output_get "User.Color" (Variables|/Script/UMG.UserWidget|GetColorAndOpacity _returnvalue_2))
            (Transformation|SetWorldScale3D _output_get (Math|Conversions|ToVector(Float) (* (Variables|/Script/TheUndoing.PaintWidget|GetBrushSize _returnvalue_2) 2e+02))))
          (:Is%20Not%20Valid
            (Development|PrintString "BP_MagicianPlayerController: ERROR spawning TrailComponent" true true "(R=1.000000,G=0.000000,B=0.031658,A=1.000000)" 1e+01)))))
    (:then_1
      (bind _returnvalue_4 (Niagara|SpawnSystemAttached (Variables|Default|GetDrawPointSystem) _rootcomponent "None" "0, 0, 0" "0, 0, 0" "KeepRelativeOffset" false false))
      (bind _output_get_2 (Variables|Default|SetDrawPointComponent _returnvalue_4))
      (Utilities|IsValid _output_get_2
        (:Is%20Valid
          (Transformation|SetWorldScale3D _output_get_2 (Math|Conversions|ToVector(Float) _spelldrawscale))
          (Effects|Components|ParticleSystem|SetFloatParameter _output_get_2 "User.Scale" _spelldrawscale))
        (:Is%20Not%20Valid
          (Development|PrintString "BP_MagicianPlayerController: ERROR spawning PointComponent" true true "(R=1.000000,G=0.000000,B=0.031658,A=1.000000)" 1e+01))))
    (:then_2
      (CallFunction|SpellDrawSetActive false))))

(fn SpellDrawSetActive
  (params (IsActive :type Boolean))
  (bind _drawpointcomponent (Variables|Default|GetDrawPointComponent))
  (bind _drawtrailcomponent (Variables|Default|GetDrawTrailComponent))
  (Utilities|FlowControl|Sequence
    (:then_0
      (bind _isusingribbon (CallFunction|IsUsingRibbon))
      (if _isusingribbon
        (Utilities|IsValid _drawtrailcomponent
          (:Is%20Valid
            (if IsActive
              (Components|Activation|Activate _drawtrailcomponent true)
              (bind _mousepos (CallFunction|GetMouseonScreenPos))
              (Transformation|SetWorldLocation _drawtrailcomponent _mousepos false true)
              (else
                (Niagara|ReinitializeSystem _drawtrailcomponent)
                (Components|Activation|Deactivate _drawtrailcomponent)))))))
    (:then_1
      (Utilities|IsValid _drawpointcomponent
        (:Is%20Valid
          (if IsActive
            (Components|Activation|Activate _drawpointcomponent true)
            (else
              (Components|Activation|Deactivate _drawpointcomponent))))))
    (:then_2
      (if (not IsActive)
        ;[0.15 0.15 0.15 0.5] Spawns poofs when done
        (for _array_element (Variables|Default|GetPoofPositions)
          (bind _returnvalue (Niagara|SpawnSystematLocation "/Game/TheUndoing/FX/SpellDrawing/NS_Poof.NS_Poof" _array_element "0, 0, 0" (Math|Conversions|ToVector(Float) (Variables|Default|GetSpellDrawScale)) true true "AutoRelease"))
          (Effects|Components|ParticleSystem|SetColorParameter _returnvalue "User.Color" (Variables|/Script/UMG.UserWidget|GetColorAndOpacity (Class|MagicianPlayerController|GetPaintWidget)))
          (Audio|PlaySound2D "/Engine/VREditor/Sounds/UI/Teleport_Committed.Teleport_Committed" 0.005 1.0 0.0 0 0))
        (Utilities|Array|Clear (Variables|Default|GetPoofPositions))))))

(fn SpellDrawUpdate
  (bind _drawtrailcomponent (Variables|Default|GetDrawTrailComponent))
  (bind _poofpositions (Variables|Default|GetPoofPositions))
  (bind _drawpointcomponent (Variables|Default|GetDrawPointComponent))
  (if (Variables|Default|GetbIsPaintingMode)
    (bind _mousepos (CallFunction|GetMouseonScreenPos))
    (Utilities|FlowControl|Sequence
      (:then_0
        (bind _isusingribbon (CallFunction|IsUsingRibbon))
        (if _isusingribbon
          (Utilities|IsValid _drawtrailcomponent
            (:Is%20Valid
              (Effects|Components|ParticleSystem|SetVectorParameter _drawtrailcomponent "User.SpawnPoint" _mousepos))
            (:Is%20Not%20Valid
              (Development|PrintString "DrawTrail is not Valid Update")))))
      (:then_1
        (Utilities|IsValid _drawpointcomponent
          (:Is%20Valid
            (Transformation|SetWorldLocation _drawpointcomponent _mousepos false true))))
      (:then_2
        ;[0.15 0.15 0.15 0.5] Remember points for poofs
        (if (Utilities|Array|IsEmpty _poofpositions)
          (bind _output_get (Variables|Default|SetSpellDrawPrevPos _mousepos :!label _label))
          (Utilities|Array|Add _poofpositions _output_get)
          (elif (not (Utilities|Operators|EqualEqual _mousepos (Variables|Default|GetSpellDrawPrevPos) 3.0))
            (goto _label)))))))

(fn EndNiagaraTrail
  (bind _isusingribbon (CallFunction|IsUsingRibbon))
  (Utilities|FlowControl|Sequence
    (:then_0
      (if _isusingribbon
        _))))

(fn LastTooClose
  (params (Points :type Array%20of%20Vectors) (NewPoint :type Vector) (Tolerance :type Float%20%28double-precision%29))
  (return false))