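; Backup version of the magician player character Blueprint, handling HUD setup, input registration and a health-refill key.
; BeginPlay creates WBP_HUD, binds it to the player's stats and the enemy found by GetActorOfClass, then adds it collapsed.
; Enhanced Input mapping is added only when an enemy exists.
; EnemyOverlap repeats enemy binding and viewport setup without collapsing the HUD; key 2 restores full health.
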(event `self.ReceiveBeginPlay`
  (bind _returnvalue (`|CreateWidget` "/Game/UI/Widgets/WBP_HUD.WBP_HUD_C" (`GameplayStatics.GetPlayerController` 0)))
  (set `self.HUDRef` _returnvalue)
  (set `/Game/UI/Widgets/WBP_HUD.PlayerStats` (`self.StatsComp`) (`self.HUDRef`))
  (bind _returnvalue_2 (`GameplayStatics.GetActorOfClass` "/Game/Blueprints/BP_Enemy.BP_Enemy_C"))
  (`/Engine/EditorBlueprintResources/StandardMacros.IsValid` _returnvalue_2
    (:`Is Valid`
      (set `/Game/UI/Widgets/WBP_HUD.EnemyStats` (`self.GetComponentByClass` _returnvalue_2 "/Game/Blueprints/BP_StatsComponent.BP_StatsComponent_C") (`self.HUDRef`))
      (`UserWidget.AddToViewport` (`self.HUDRef`) 0)
      (`Widget.SetVisibility` (`self.HUDRef`) "Collapsed")
      (`KismetSystemLibrary.PrintString` "HUD Created")
      (`EnhancedInputSubsystemInterface.AddMappingContext` (pcsubsystem `EnhancedInputLocalPlayerSubsystem` (`GameplayStatics.GetPlayerController` 0)) null 0 (struct))
      (`KismetSystemLibrary.PrintString` "IMC Added" true true (struct :`R` 0.015711 :`G` 0.494792 :`B` 0.001651 :`A` 1.0)))
    (:`Is Not Valid`
      (`KismetSystemLibrary.PrintString` "BP_Player_No Enemy Found" true true (struct :`R` 0.463542 :`G` 0.022485 :`A` 1.0) 5.0)
      (`UserWidget.AddToViewport` (`self.HUDRef`) 0)
      (`Widget.SetVisibility` (`self.HUDRef`) "Collapsed"))))

(event `Key|Two`
  (params (Key :type "Key Structure"))
  (bind _statscomp (`self.StatsComp`))
  (:`Pressed`
    (set `/Game/Blueprints/BP_StatsComponent.CurrentHealth` (`/Game/Blueprints/BP_StatsComponent.MaxHealth` _statscomp) _statscomp)))

(event `EnemyOverlap`
  (bind _returnvalue (`GameplayStatics.GetActorOfClass` "/Game/Blueprints/BP_Enemy.BP_Enemy_C"))
  (`/Engine/EditorBlueprintResources/StandardMacros.IsValid` _returnvalue
    (:`Is Valid`
      (set `/Game/UI/Widgets/WBP_HUD.EnemyStats` (`self.GetComponentByClass` _returnvalue "/Game/Blueprints/BP_StatsComponent.BP_StatsComponent_C") (`self.HUDRef`))
      (`UserWidget.AddToViewport` (`self.HUDRef`) 0)
      (`KismetSystemLibrary.PrintString` "HUD Created")
      (`EnhancedInputSubsystemInterface.AddMappingContext` (pcsubsystem `EnhancedInputLocalPlayerSubsystem` (`GameplayStatics.GetPlayerController` 0)) null 0 (struct))
      (`KismetSystemLibrary.PrintString` "IMC Added" true true (struct :`R` 0.015711 :`G` 0.494792 :`B` 0.001651 :`A` 1.0)))
    (:`Is Not Valid`
      (`KismetSystemLibrary.PrintString` "BP_Player_No Enemy Found" true true (struct :`R` 0.463542 :`G` 0.022485 :`A` 1.0) 5.0)
      (`UserWidget.AddToViewport` (`self.HUDRef`) 0))))

(fn `UserConstructionScript`)