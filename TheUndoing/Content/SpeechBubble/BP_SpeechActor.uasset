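; BP_SpeechActor is a talkable actor that shows a prompt bubble in range and runs a text-box conversation on interact.
; Lines load from a data table, with ProgressDialouge switching to later rows.
; The player controller's interact event opens dialogue or advances lines, exiting after the last, unless UIManager is open.
; During dialogue, player movement is disabled and the view switches to a dialogue camera placed between speaker and player camera.
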(event `self.ReceiveBeginPlay`
  (bind _greetings (`self.Greetings`))
  (if (`self.IsQuestInfo`)
    (bind _aswbp_bubble (cast `/Game/SpeechBubble/WBP_Bubble` (`WidgetComponent.GetWidget` _greetings))
      (:`then`
        (`/Game/SpeechBubble/WBP_Bubble.SetText` _aswbp_bubble "!")
        (`SceneComponent.SetHiddenInGame` _greetings false true))
      (:`CastFailed`
        _)))
  (`self.LoadDialouge`)
  (set `self.Index` 0)
  (bind _aswbp_text_box (cast `/Game/SpeechBubble/WBP_TextBox` (`WidgetComponent.GetWidget` (`self.Widget`))))
  (set `TextBlock.Text` (`|GetArrayItem` (`self.SpechText`) (`self.Index`)) (`/Game/SpeechBubble/WBP_TextBox.Text` _aswbp_text_box))
  (bind _aswbp_text_box_2 (cast `/Game/SpeechBubble/WBP_TextBox` (`WidgetComponent.GetWidget` (`self.Widget`))))
  (set `TextBlock.Text` (`self.NameText`) (`/Game/SpeechBubble/WBP_TextBox.NameText` _aswbp_text_box_2))
  ; Catch IA_Interact from PlayerController
  (bind _asbp_magician_player_controller (cast `/Game/Player/BP_MagicianPlayerController` (`GameplayStatics.GetPlayerController` 0)))
  (add `/Game/Player/BP_MagicianPlayerController.OnTryInteract` _asbp_magician_player_controller (delegate `RecieveInteract`)))

(event `RecieveInteract`
  ; Catch IA_Interact from PlayerController
  (`self.Interact`))

(event `self.InteractionRadius.OnComponentBeginOverlap`
  (params (OverlappedComponent :type "PrimitiveComponent Object Reference") (OtherActor :type "Actor Object Reference") (OtherComp :type "PrimitiveComponent Object Reference") (OtherBodyIndex :type Integer) (bFromSweep :type Boolean) (SweepResult :type "HitResult Structure (by ref)"))
  (`self.Is Close` true)
  (if (`self.IsQuestInfo`)
    (set `self.IsQuestInfo` false)
    (bind _aswbp_bubble (cast `/Game/SpeechBubble/WBP_Bubble` (`WidgetComponent.GetWidget` (`self.Greetings`))))
    (`/Game/SpeechBubble/WBP_Bubble.SetText` _aswbp_bubble "Press E")))

(event `self.InteractionRadius.OnComponentEndOverlap`
  (params (OverlappedComponent :type "PrimitiveComponent Object Reference") (OtherActor :type "Actor Object Reference") (OtherComp :type "PrimitiveComponent Object Reference") (OtherBodyIndex :type Integer))
  (`self.Is Close` false))

(fn `EnterDialouge`
  (bind _returnvalue (`self.K2_GetActorLocation`))
  (bind _returnvalue_2 (`GameplayStatics.GetPlayerCharacter` 0))
  (bind _dialoguecamera (`self.DialogueCamera`))
  (set `self.IsActive` true)
  (`CharacterMovementComponent.DisableMovement` (`Character.CharacterMovement` _returnvalue_2))
  (bind _asbp_magician_player_character (cast `/Game/Player/BP_MagicianPlayerCharacter` _returnvalue_2))
  (bind _camera (`/Game/Player/BP_MagicianPlayerCharacter.Camera` _asbp_magician_player_character))
  (`SceneComponent.K2_SetWorldLocationAndRotation` _dialoguecamera (+ (* (- (`SceneComponent.K2_GetComponentLocation` _camera) _returnvalue) 0.3) _returnvalue) (`SceneComponent.K2_GetComponentRotation` _camera) false true)
  (`SceneComponent.K2_AddLocalRotation` _dialoguecamera (struct :`Pitch` -10.0) false false)
  (bind _aswbp_text_box (cast `/Game/SpeechBubble/WBP_TextBox` (`WidgetComponent.GetWidget` (`self.Widget`))))
  (`UserWidget.AddToViewport` _aswbp_text_box 0)
  (`self.SwitchCam`)
  (`SceneComponent.SetHiddenInGame` (`self.Greetings`) true false)
  (bind _asbp_magician_player_character_2 (cast `/Game/Player/BP_MagicianPlayerCharacter` (`GameplayStatics.GetPlayerCharacter` 0)))
  (set `/Game/Player/BP_MagicianPlayerCharacter.InConvo` true _asbp_magician_player_character_2))

(fn `ExitDialouge`
  (`CharacterMovementComponent.SetMovementMode` (`Character.CharacterMovement` (`GameplayStatics.GetPlayerCharacter` 0)) "MOVE_Walking" 0)
  (set `self.IsActive` false)
  (`Widget.RemoveFromParent` (`WidgetComponent.GetWidget` (`self.Widget`)))
  (`self.SwitchCam`)
  (`SceneComponent.SetHiddenInGame` (`self.Greetings`) false false)
  (bind _asbp_magician_player_character (cast `/Game/Player/BP_MagicianPlayerCharacter` (`GameplayStatics.GetPlayerCharacter` 0)))
  (set `/Game/Player/BP_MagicianPlayerCharacter.InConvo` false _asbp_magician_player_character))

(fn `Increment Index`
  (returns (ReadAll :type Boolean))
  (bind _result (`/Engine/EditorBlueprintResources/StandardMacros.IncrementInt` (`self.Index`))
    (:`  `
      (bind _returnvalue (> _result (- (`KismetArrayLibrary.Array_Length` (`self.SpechText`)) 1)))
      (if _returnvalue
        (set `self.Index` 0))
      (bind _aswbp_text_box (cast `/Game/SpeechBubble/WBP_TextBox` (`WidgetComponent.GetWidget` (`self.Widget`))))
      (set `TextBlock.Text` (`|GetArrayItem` (`self.SpechText`) (`self.Index`)) (`/Game/SpeechBubble/WBP_TextBox.Text` _aswbp_text_box))
      (return _returnvalue))))

(fn `Interact`
  (bind _returnvalue (`GameplayStatics.GetActorOfClass` "/Game/UI/Systems/UIManager.UIManager_C"))
  (if (`/Game/UI/Systems/UIManager.IsOpen` _returnvalue)
    _
    (elif (`self.InRange`)
      (if (`self.IsActive`)
        (bind _readall (`self.Increment Index`))
        (if _readall
          (`self.ExitDialouge`))
        (else
          (`self.EnterDialouge`))))))

(fn `Is Close`
  (params (InRange :type Boolean))
  (bind _output_get (set `self.InRange` InRange))
  (`SceneComponent.SetHiddenInGame` (`self.Greetings`) (not _output_get) false))

(fn `LoadDialouge`
  (bind _dialougedatatable (`self.DialougeDataTable`))
  (`/Engine/EditorBlueprintResources/StandardMacros.IsValid` _dialougedatatable
    (:`Is Valid`
      (bind _outrownames (`DataTableFunctionLibrary.GetDataTableRowNames` _dialougedatatable))
      (bind _output_get (set `self.DTRowNames` _outrownames))
      (bind _returnvalue (`|GetDataTableRow` _dialougedatatable (`|GetArrayItem` _output_get))
        (:`then`
          (set `self.SpechText` (`.Lines_12_D9ED3B034BD8D01EE85626AA44ADF759` (break `/Game/SpeechBubble/Dialouges/S_Dialouge` _returnvalue))))
        (:`RowNotFound`
          (`KismetSystemLibrary.PrintString` "ERROR: (BP_SpeechActor) Error loading dialouge table" false true (struct :`R` 1.0 :`G` 0.007137 :`A` 1.0) 5.0))))))

(fn `ProgressDialouge`
  (bind _dialougedatatable (`self.DialougeDataTable`))
  (bind _dtrowindex (`self.DTRowIndex`))
  (`/Engine/EditorBlueprintResources/StandardMacros.IsValid` _dialougedatatable
    (:`Is Valid`
      (if (> (`KismetArrayLibrary.Array_Length` (`self.DTRowNames`)) (- 1 _dtrowindex))
        (bind _result (`/Engine/EditorBlueprintResources/StandardMacros.IncrementInt` _dtrowindex)
          (:`  `
            (bind _returnvalue (`|GetDataTableRow` _dialougedatatable (`|GetArrayItem` (`self.DTRowNames`) _result))
              (:`then`
                (set `self.SpechText` (`.Lines_12_D9ED3B034BD8D01EE85626AA44ADF759` (break `/Game/SpeechBubble/Dialouges/S_Dialouge` _returnvalue)))
                (set `self.Index` -1)
                (`self.Increment Index`)))))))
    (:`Is Not Valid`
      (`KismetSystemLibrary.PrintString` "ERROR: (BP_SpeechActor) Error loading dialouge table" false true (struct :`R` 1.0 :`G` 0.007137 :`A` 1.0) 5.0))))

(fn `SwitchCam`
  (locals (NewCamera :type "Actor Object Reference"))
  (if (`self.IsActive`)
    (set `local.NewCamera` self)
    (else
      (set `local.NewCamera` (`GameplayStatics.GetPlayerCharacter` 0))))
  (`PlayerController.SetViewTargetWithBlend` (`GameplayStatics.GetPlayerController` 0) (`local.NewCamera`) 0.0 "VTBlend_Linear" 0.0 false))

(fn `UserConstructionScript`)