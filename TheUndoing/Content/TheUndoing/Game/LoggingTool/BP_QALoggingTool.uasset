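; BP_QALoggingTool is a QA logging tool that records recognized spell casts to a saved log file.
; BindSpellEvent binds to the player controller's OnSpellRecognized event, passing each result to HandleSpellCast.
; HandleSpellCast appends a comma-separated line of spell name, success and score to the file at CurLogPath.
; The session, counter, event log and flush functions are empty stubs.
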(event `BindSpellEvent`
  (`KismetSystemLibrary.PrintString` null "Initialize Logging tool")
  (add `MagicianPlayerController.OnSpellRecognized` (`self.PlayerControllerRef`) (delegate `LogRecognizedSpell`)))

(event `LogRecognizedSpell`
  (params (Result :type "SpellRecognitionResult Structure (by ref)"))
  (`KismetSystemLibrary.PrintString` null "Should log spell")
  (`self.HandleSpellCast` Result))

(fn `ClearLog`)

(fn `FlushToDisk`)

(fn `GetAllCounters`)

(fn `GetCounter`)

(fn `GetEvents`)

(fn `HandleSpellCast`
  (params (SpellData :type "SpellRecognitionResult Structure"))
  (`LogFileParser.AppendLineToSavedLogFile` (`self.CurLogPath`) (`KismetStringLibrary.Concat_StrStr` SpellData_Name "," (`KismetStringLibrary.Conv_BoolToString` SpellData_bSuccess) "," (`KismetStringLibrary.Conv_DoubleToString` SpellData_Score)))
  (return))

(fn `IncrementCounter`)

(fn `InitializeSession`)

(fn `LogEvent`)

(fn `SetCounter`)