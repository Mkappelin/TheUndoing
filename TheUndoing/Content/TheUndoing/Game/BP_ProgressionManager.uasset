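; Progression manager for The Undoing that tracks which spells the player has learned and how many cleanses have been counted.
; Setup fills the full spell list from the spell enum and copies it into the available pool.
; UnlockSpell moves a spell from available to learned, or prints an already-learned message and returns false.
; Simple getters expose the cleansed count and the spell lists.
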(event `Setup`
  (bind _enumvalue (foreach `/Game/Blueprints/Spells` false)
    (:`LoopBody`
      (`KismetArrayLibrary.Array_AddUnique` (`self.AllSpells`) _enumvalue))
    (:`then`
      (`KismetArrayLibrary.Array_Append` (`self.AvaliableSpells`) (`self.AllSpells`)))))

(fn `AddOneCleansed`
  (`/Engine/EditorBlueprintResources/StandardMacros.IncrementInt` (`self.number_of_cleansed`)))

(fn `GetAllSpells`
  (returns (Spells :type "Array of /Game/Blueprints/Spells Enum"))
  (return (`self.AllSpells`)))

(fn `GetCleansed`
  (returns (NumOfCleansed :type Integer))
  (return (`self.number_of_cleansed`)))

(fn `GetLearnedSpells`
  (returns (Spells :type "Array of /Game/Blueprints/Spells Enum"))
  (return (`self.SpellsLearned`)))

(fn `UnlockSpell`
  (params (SpellToUnlock :type "/Game/Blueprints/Spells Enum" :default "NewEnumerator0"))
  (returns (WasNew :type Boolean))
  (if (`KismetArrayLibrary.Array_Contains` (`self.AvaliableSpells`) SpellToUnlock)
    (`KismetArrayLibrary.Array_AddUnique` (`self.SpellsLearned`) SpellToUnlock)
    (`KismetArrayLibrary.Array_RemoveItem` (`self.AvaliableSpells`) SpellToUnlock)
    (return true)
    (else
      (`KismetSystemLibrary.PrintString` null (`KismetStringLibrary.Concat_StrStr` "UDefaultGameInstance: " (`|GetEnumeratorNameAsString` SpellToUnlock) " Spell already learned") true true (struct :`R` 1.0 :`B` 0.015603 :`A` 1.0))
      (return false))))