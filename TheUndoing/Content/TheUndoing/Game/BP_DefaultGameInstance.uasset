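; Game instance for The Undoing that owns the save, level-flow, progression and QA logging manager objects, all constructed on Init.
; After a two-second delay it caches the magician character and controller, binds spell logging and creates a QA log file.
; It stores an entry tag for level travel, teleports the player to the matching travel point, and forwards spell checks and unlocks to the progression manager.
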(event `self.ReceiveInit`
  (`|ExecutionSequence`
    (:`then_0`
      (bind _returnvalue (`|GenericCreateObject` self "/Game/TheUndoing/Game/BP_SaveManager.BP_SaveManager_C"))
      (set `self.SaveManager` _returnvalue))
    (:`then_1`
      (bind _returnvalue_2 (`|GenericCreateObject` self "/Game/TheUndoing/Game/BP_LevelFlowManager.BP_LevelFlowManager_C"))
      (set `self.LevelFlowManager` _returnvalue_2))
    (:`then_2`
      (bind _returnvalue_3 (`|GenericCreateObject` self "/Game/TheUndoing/Game/BP_ProgressionManager.BP_ProgressionManager_C"))
      (bind _output_get (set `self.ProgressionManager` _returnvalue_3))
      (`/Game/TheUndoing/Game/BP_ProgressionManager.Setup` _output_get))
    (:`then_3`
      (bind _returnvalue_4 (`|GenericCreateObject` self "/Game/TheUndoing/Game/LoggingTool/BP_QALoggingTool.BP_QALoggingTool_C"))
      (set `self.LoggingTool` _returnvalue_4))
    (:`then_4`
      ; (Do in player init later)
      (`KismetSystemLibrary.Delay` 2.0)
      (`self.AssignPlayer`)
      ; Initial QA-log creation
      (bind (_outfullpath _returnvalue_5) (`LogFileParser.CreateLogFile` "QA_Logs"))
      (if _returnvalue_5
        (bind _output_get_2 (set `/Game/TheUndoing/Game/LoggingTool/BP_QALoggingTool.CurLogPath` _outfullpath (`self.LoggingTool`)))
        (`KismetSystemLibrary.PrintString` (`KismetStringLibrary.Concat_StrStr` "Log was successfully created at: " _output_get_2) false true (struct :`R` 0.024743 :`G` 1.0 :`A` 1.0) 10.0)
        (else
          (`KismetSystemLibrary.PrintString` "Log creation failed!!!" false true (struct :`R` 1.0 :`G` 0.010018 :`A` 1.0) 10.0))))))

(event `self.ReceiveShutdown`)

(fn `AssignPlayer`
  (locals (PCharacter :type "/Game/Player/BP_MagicianPlayerCharacter Object Reference") (PController :type "/Game/Player/BP_MagicianPlayerController Object Reference"))
  (bind _loggingtool (`self.LoggingTool`))
  (bind _asbp_magician_player_character (cast `/Game/Player/BP_MagicianPlayerCharacter` (`GameplayStatics.GetPlayerCharacter` 0)))
  (set `local.PCharacter` _asbp_magician_player_character)
  (bind _asbp_magician_player_controller (cast `/Game/Player/BP_MagicianPlayerController` (`GameplayStatics.GetPlayerController` 0)))
  (set `local.PController` _asbp_magician_player_controller)
  (set `/Game/TheUndoing/Game/LoggingTool/BP_QALoggingTool.PlayerCharacterRef` (`local.PCharacter`) _loggingtool)
  (set `/Game/TheUndoing/Game/LoggingTool/BP_QALoggingTool.PlayerControllerRef` (`local.PController`) _loggingtool)
  (`/Game/TheUndoing/Game/LoggingTool/BP_QALoggingTool.BindSpellEvent` _loggingtool))

(fn `CloseGame`
  (`KismetSystemLibrary.QuitGame` (`GameplayStatics.GetPlayerController` 0) "Quit"))

(fn `LogSpell`
  (params (SpellData :type "SpellRecognitionResult Structure")))

(fn `NewFunction`
  (returns (NewParam :type Boolean))
  (return false))

(fn `PlacePlayerAtEntryPoint`
  (bind _outactors (`GameplayStatics.GetAllActorsOfClass` "/Game/TheUndoing/Objects/BP_LevelTravelPoint.BP_LevelTravelPoint_C"))
  (for _array_element _outactors
    (if (== (`self.PendingEntryTag`) (`/Game/TheUndoing/Objects/BP_LevelTravelPoint.EntryTag` _array_element))
      (bind _entrypoint (`/Game/TheUndoing/Objects/BP_LevelTravelPoint.EntryPoint` _array_element))
      (`Actor.K2_TeleportTo` (`GameplayStatics.GetPlayerCharacter` 0) (`SceneComponent.K2_GetComponentLocation` _entrypoint) (`SceneComponent.K2_GetComponentRotation` _entrypoint))
      (return)))
  (`KismetSystemLibrary.PrintString` "GameInstance: Could not find level entry point" true true (struct :`R` 1.0 :`G` 0.604552 :`A` 1.0) 5.0))

(fn `PlayerHasSpell`
  (params (Spell :type "/Game/Blueprints/Spells Enum" :default "NewEnumerator0"))
  (returns (HasSpell :type Boolean))
  (bind _spells (`/Game/TheUndoing/Game/BP_ProgressionManager.GetLearnedSpells` (`self.ProgressionManager`)))
  (return (`KismetArrayLibrary.Array_Contains` _spells Spell)))

(fn `TravelToLevel`
  (params (LevelName :type Name) (EntryTag :type Name))
  (set `self.PendingLevelName` LevelName)
  (set `self.PendingEntryTag` EntryTag)
  (`GameplayStatics.OpenLevel` (`self.PendingLevelName`)))

(fn `UnlockSpell`
  (params (NewSpell :type "/Game/Blueprints/Spells Enum" :default "NewEnumerator0"))
  (returns (Success :type Boolean))
  (bind _wasnew (`/Game/TheUndoing/Game/BP_ProgressionManager.UnlockSpell` (`self.ProgressionManager`) NewSpell))
  (return _wasnew))