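; BP_LevelTravelPoint is a level transition actor that sends the magician player to a target level and serves as the arrival point from it.
; Overlap passes the target level and current level name, as entry tag, to BP_DefaultGameInstance's TravelToLevel.
; Shortly after BeginPlay, the point whose target matches the pending entry tag teleports the player to its EntryPoint, so return links need no separate IDs.
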(event `self.ReceiveBeginPlay`
  (bind _returnvalue (`GameplayStatics.GetCurrentLevelName` true))
  (set `self.EntryTag` (`KismetStringLibrary.Conv_StringToName` _returnvalue))
  (`KismetSystemLibrary.Delay` 0.01)
  (bind _asbp_default_game_instance (cast `/Game/TheUndoing/Game/BP_DefaultGameInstance` (`GameplayStatics.GetGameInstance`)))
  (if (== (`/Game/TheUndoing/Game/BP_DefaultGameInstance.PendingEntryTag` _asbp_default_game_instance) (`self.TargetLevelName`))
    (`self.TeleportPlayerHere`)))

(event `self.ReceiveActorBeginOverlap`
  (params (OtherActor :type "Actor Object Reference"))
  (cast `/Game/Player/BP_MagicianPlayerCharacter` OtherActor)
  (bind _asbp_default_game_instance (cast `/Game/TheUndoing/Game/BP_DefaultGameInstance` (`GameplayStatics.GetGameInstance`))
    (:`then`
      (`/Game/TheUndoing/Game/BP_DefaultGameInstance.TravelToLevel` _asbp_default_game_instance (`self.TargetLevelName`) (`self.EntryTag`)))
    (:`CastFailed`
      (`KismetSystemLibrary.PrintString` "Why are we still here? just to suffer?"))))

(fn `TeleportPlayerHere`
  (bind _returnvalue (`GameplayStatics.GetPlayerCharacter` 0))
  (bind _entrypoint (`self.EntryPoint`))
  (bind _returnvalue_2 (`SceneComponent.K2_GetComponentLocation` _entrypoint))
  (`KismetSystemLibrary.PrintString` "Player and location: " true true (struct :`G` 0.66 :`B` 1.0 :`A` 1.0) 10.0)
  (`KismetSystemLibrary.PrintString` (`KismetSystemLibrary.GetDisplayName` _returnvalue) true true (struct :`G` 0.66 :`B` 1.0 :`A` 1.0) 10.0)
  (`KismetSystemLibrary.PrintString` (`KismetStringLibrary.Conv_VectorToString` _returnvalue_2) true true (struct :`G` 0.66 :`B` 1.0 :`A` 1.0) 10.0)
  (`self.K2_TeleportTo` _returnvalue _returnvalue_2 (`SceneComponent.K2_GetComponentRotation` _entrypoint)))

(fn `UserConstructionScript`)